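; Easter basket actor for an egg hunt that collects BP_EasterEgg actors and tracks progress toward six.
; An egg entering the Box plays a pop sound, and a MultiGate reveals the next static mesh, increments the count and destroys the egg.
; A looping half-second timer updates a text render tally, then stops itself and plays a victory sound once all six are in.
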(event OnComponentBeginOverlap(Box)
  (params (OverlappedComponent :type Primitive%20Component%20Object%20Reference) (OtherActor :type Actor%20Object%20Reference) (OtherComp :type Primitive%20Component%20Object%20Reference) (OtherBodyIndex :type Integer) (bFromSweep :type Boolean) (SweepResult :type Hit%20Result%20Structure%20%28by%20ref%29))
  (bind _array_index (Variables|Default|GetArray%20Index))
  (bind _asbp_easter_egg (Utilities|Casting|CastToBP_EasterEgg OtherActor))
  (Audio|PlaySound2D "/Game/VRE/Blueprints/ChristmasTree/PopSound.PopSound" 1.0 1.0 0.0 0 0)
  (Utilities|FlowControl|MultiGate false false _array_index
    (:Out%200
      (Rendering|SetVisibility (Variables|Default|GetStaticMesh1) true false)
      (Math|Integer|IncrementInt _array_index
        (:%20%20
          (Actor|DestroyActor _asbp_easter_egg))))
    (:Out%201
      (Rendering|SetVisibility (Variables|Default|GetStaticMesh5) true false)
      (Math|Integer|IncrementInt _array_index
        (:%20%20
          (Actor|DestroyActor _asbp_easter_egg))))
    (:Out%202
      (Rendering|SetVisibility (Variables|Default|GetStaticMesh4) true false)
      (Math|Integer|IncrementInt _array_index
        (:%20%20
          (Actor|DestroyActor _asbp_easter_egg))))
    (:Out%203
      (Rendering|SetVisibility (Variables|Default|GetStaticMesh2) true false)
      (Math|Integer|IncrementInt _array_index
        (:%20%20
          (Actor|DestroyActor _asbp_easter_egg))))
    (:Out%204
      (Rendering|SetVisibility (Variables|Default|GetStaticMesh3) true false)
      (Math|Integer|IncrementInt _array_index
        (:%20%20
          (Actor|DestroyActor _asbp_easter_egg))))
    (:Out%205
      (Rendering|SetVisibility (Variables|Default|GetStaticMesh) true false)
      (Math|Integer|IncrementInt _array_index
        (:%20%20
          (Actor|DestroyActor _asbp_easter_egg))))))

(event Custom|Update%20Tally
  (Rendering|Components|TextRender|SetText (Variables|Default|GetTextRender) (Utilities|Text|ToText(String) (Utilities|String|Append (Utilities|String|ToString(Integer) (Variables|Default|GetArray%20Index)) "/" "6")))
  (if (>= (Variables|Default|GetArray%20Index) 6)
    (Utilities|Time|ClearandInvalidateTimerbyHandle (stale EventBeginPlay _returnvalue))
    (Audio|PlaySound2D "/Game/VRE/SFX/Victory/victory.victory" 1.0 1.0 0.0 0 0)))

(event Collision|EventActorBeginOverlap
  (params (OtherActor :type Actor%20Object%20Reference)))

(event EventTick
  (params (DeltaSeconds :type Float%20%28single-precision%29)))

(event EventBeginPlay
  (bind _returnvalue (Utilities|Time|SetTimerbyEvent (delegate Custom|Update%20Tally) 0.5 true)))

(fn ConstructionScript)