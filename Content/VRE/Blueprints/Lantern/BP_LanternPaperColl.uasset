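; Collectible lantern paper pickup for a VR game that counts toward the pages collected on BP_LanternMain.
; A timeline spins it while a sine offset bobs it vertically.
; When a VRBaseCharacter overlaps its box, it plays a sound, increments the count, disables collision, spins faster, then rises and destroys itself.
; An unconnected MultiGate for revealing lantern frame stages remains in the graph but never runs.
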(event OnComponentBeginOverlap(Box)
  (params (OverlappedComponent :type Primitive%20Component%20Object%20Reference) (OtherActor :type Actor%20Object%20Reference) (OtherComp :type Primitive%20Component%20Object%20Reference) (OtherBodyIndex :type Integer) (bFromSweep :type Boolean) (SweepResult :type Hit%20Result%20Structure%20%28by%20ref%29))
  (Utilities|Casting|CastToVRBaseCharacter OtherActor)
  (CallFunction|PageCollected))

(event Custom|PageCollected
  (Audio|PlaySound2D "/Game/VRE/Blueprints/Lantern/SFX/Pickup1.Pickup1" 1.0 1.0 0.0 0 0)
  (bind _outactors (Actor|GetAllActorsOfClass "/Game/VRE/Blueprints/Lantern/BP_LanternMain.BP_LanternMain_C"))
  (Math|Integer|IncrementInt (Variables|/Game/VRE/Blueprints/Lantern/BP_LanternMain.BP_LanternMain_C|GetPagesCollected (Utilities|Array|Get(acopy) _outactors))
    (:%20%20
      (Collision|SetCollisionEnabled (Variables|Default|GetBox) "NoCollision")
      (Variables|Default|SetRot 5e+03)
      (Utilities|FlowControl|Delay 1.0)
      (Audio|PlaySound2D "/Game/VRE/Blueprints/Lantern/SFX/Airmove.Airmove" 1.0 1.0 0.0 0 0)
      (Components|Timeline|SetPlayRate (Variables|Default|GetTL_UP) (/ 1.0 (Variables|Default|GetTimeline%20Length_UP)))
      (bind _alpha (Timeline|TL_UP Play)
        (:Update
          (Transformation|AddActorWorldOffset (Math|Vector|MakeVector 0.0 0.0 (* _alpha 1e+02)))
          (Utilities|FlowControl|Delay 2.0)
          (Actor|DestroyActor))))))

(event EventBeginPlay
  (Components|Timeline|SetPlayRate (Variables|Default|GetTL_Rotation) (/ 1.0 (Variables|Default|GetTimeline%20Length_Rot)))
  (bind _alpha (Timeline|TL_Rotation PlayFromStart)
    (:Update
      (Transformation|SetActorRelativeRotation (Math|Rotator|MakeRotator 0.0 9e+01 (* _alpha (Variables|Default|GetRot))))
      (Transformation|AddActorWorldOffset (Math|Vector|MakeVector 0.0 0.0 (* (* (Math|Trig|Sin(Degrees) (* (Utilities|Time|GetGameTimeinSeconds) 5e+01)) 0.01111) 1e+01))))))

(event EventOnUsed)

(fn ConstructionScript)