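; VR lantern actor that the player assembles from paper, flower and candle pieces, then lights and launches.
; Capsule overlaps with those pieces toggle Interacting, while a looping timer spawns a lantern paper at a preset spot for each PagesCollected milestone, stopping after the last.
; Using the completed lantern releases the character's grips, ignites the flame and starts timelines that drift and spin it with gravity off; incomplete use plays a denial sound.
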(event OnComponentBeginOverlap(Capsule)
  (params (OverlappedComponent :type Primitive%20Component%20Object%20Reference) (OtherActor :type Actor%20Object%20Reference) (OtherComp :type Primitive%20Component%20Object%20Reference) (OtherBodyIndex :type Integer) (bFromSweep :type Boolean) (SweepResult :type Hit%20Result%20Structure%20%28by%20ref%29))
  (Utilities|FlowControl|Sequence
    (:then_0
      (Utilities|Casting|CastToBP_LanternPaper OtherActor))
    (:then_1
      (Utilities|Casting|CastToBP_FlowerLantern OtherActor))
    (:then_2
      (Utilities|Casting|CastToBP_CandleLantern OtherActor)))
  (Variables|Default|Setinteracting true))

(event OnComponentEndOverlap(Capsule)
  (params (OverlappedComponent :type Primitive%20Component%20Object%20Reference) (OtherActor :type Actor%20Object%20Reference) (OtherComp :type Primitive%20Component%20Object%20Reference) (OtherBodyIndex :type Integer))
  (Utilities|FlowControl|Sequence
    (:then_0
      (Utilities|Casting|CastToBP_LanternPaper OtherActor))
    (:then_1
      (Utilities|Casting|CastToBP_FlowerLantern OtherActor))
    (:then_2
      (Utilities|Casting|CastToBP_CandleLantern OtherActor)))
  (Variables|Default|Setinteracting false))

(event Custom|Lantern%20Flight
  (Physics|SetEnableGravity (Variables|Default|GetStaticMeshComponent) false)
  (Components|Timeline|SetPlayRate (Variables|Default|GetTL_Lantern) (/ 1.0 (Variables|Default|GetTimeline%20Length)))
  (Timeline|TL_Lantern PlayFromStart
    (:Update
      (Transformation|SetActorLocation (+ (Transformation|GetActorLocation) (* (Math|Vector|GetForwardVector (Variables|Default|GetArrow)) 0.5)) false false)
      (Components|Timeline|SetPlayRate (Variables|Default|GetTL_Rot) (/ 1.0 (Variables|Default|GetTimeline%20Length_0)))
      (bind _alpha (Timeline|TL_Rot Play)
        (:Update
          (Transformation|SetActorRelativeRotation (Math|Rotator|MakeRotator -1.8e+02 0.0 (* _alpha 3.6e+02))))))))

(event Custom|PageCheck
  (Utilities|FlowControl|Sequence
    (:then_0
      (if (== (Variables|Default|GetPagesCollected) 1)
        (Utilities|FlowControl|DoOnce false
          (:Completed
            (Game|SpawnActorfromClass "/Game/VRE/Blueprints/Lantern/BP_LanternPaper.BP_LanternPaper_C" (Math|Transform|MakeTransform (Variables|Default|GetSpawn%20Transform%20Location%201%20) "90.000000,1620.000000,0.000000" (Variables|Default|GetSpawn%20Transform%20Scale)) "Undefined" "MultiplyWithRoot" 0 0)))))
    (:then_1
      (if (== (Variables|Default|GetPagesCollected) 2)
        (Utilities|FlowControl|DoOnce false
          (:Completed
            (Game|SpawnActorfromClass "/Game/VRE/Blueprints/Lantern/BP_LanternPaper.BP_LanternPaper_C" (Math|Transform|MakeTransform (Variables|Default|GetSpawn%20Transform%20Location%202) "90.000000,3870.000000,0.000000" (Variables|Default|GetSpawn%20Transform%20Scale)) "Undefined" "MultiplyWithRoot" 0 0)))))
    (:then_2
      (if (== (Variables|Default|GetPagesCollected) 3)
        (Utilities|FlowControl|DoOnce false
          (:Completed
            (Game|SpawnActorfromClass "/Game/VRE/Blueprints/Lantern/BP_LanternPaper.BP_LanternPaper_C" (Math|Transform|MakeTransform (Variables|Default|GetSpawn%20Transform%20Location%203) "90.000000,-165.000000,0.000000" (Variables|Default|GetSpawn%20Transform%20Scale)) "Undefined" "MultiplyWithRoot" 0 0)))))
    (:then_3
      (if (== (Variables|Default|GetPagesCollected) 4)
        (Utilities|FlowControl|DoOnce false
          (:Completed
            (Game|SpawnActorfromClass "/Game/VRE/Blueprints/Lantern/BP_LanternPaper.BP_LanternPaper_C" (Math|Transform|MakeTransform (Variables|Default|GetSpawn%20Transform%20Location%204) "90.000000,180.000000,0.000000" (Variables|Default|GetSpawn%20Transform%20Scale)) "Undefined" "MultiplyWithRoot" 0 0)))))
    (:then_4
      (if (== (Variables|Default|GetPagesCollected) 5)
        (Utilities|FlowControl|DoOnce false
          (:Completed
            (Game|SpawnActorfromClass "/Game/VRE/Blueprints/Lantern/BP_LanternPaper.BP_LanternPaper_C" (Math|Transform|MakeTransform (Variables|Default|GetSpawn%20Transform%20Location%205) "90.000000,1106.000000,0.000000" (Variables|Default|GetSpawn%20Transform%20Scale)) "Undefined" "MultiplyWithRoot" 0 0)))))
    (:then_5
      (if (== (Variables|Default|GetPagesCollected) 6)
        (Utilities|FlowControl|DoOnce false
          (:Completed
            (Utilities|Time|ClearandInvalidateTimerbyHandle (stale EventBeginPlay _returnvalue))
            (Game|SpawnActorfromClass "/Game/VRE/Blueprints/Lantern/BP_LanternPaper.BP_LanternPaper_C" (Math|Transform|MakeTransform (Variables|Default|GetSpawn%20Transform%20Location%206) "90.000000,1953.000000,0.000000" (Variables|Default|GetSpawn%20Transform%20Scale)) "Undefined" "MultiplyWithRoot" 0 0)))))))

(event EventOnGripRelease
  (params (ReleasingController :type Grip%20Motion%20Controller%20Component%20Object%20Reference) (GripInformation :type BP%20Actor%20Grip%20Information%20Structure%20%28by%20ref%29) (bWasSocketed :type Boolean))
  (if (Variables|Default|GetCandle%20Activated)
    _))

(event Collision|EventActorBeginOverlap
  (params (OtherActor :type Actor%20Object%20Reference)))

(event EventBeginPlay
  (bind _returnvalue (Utilities|Time|SetTimerbyEvent (delegate Custom|PageCheck) 1.0 true)))

(event EventOnUsed
  (if (Math|Boolean|ANDBoolean (Variables|Default|Getframe%20built%20main) (Variables|Default|GetFlower%20Built) (Variables|Default|GetCandle%20Built))
    (Variables|Default|SetCandle%20Activated true)
    (bind _outactors (Actor|GetAllActorsOfClass "/Game/VRE/Core/Character/BP_VRCharacter.BP_VRCharacter_C"))
    (Utilities|FlowControl|Sequence
      (:then_0
        (bind _griparray (Class|GripMotionControllerComponent|GetAllGrips (Variables|/Script/VRExpansionPlugin.VRBaseCharacter|GetLeftMotionController (Utilities|Array|Get(acopy) _outactors))))
        (for _array_element _griparray
          (Class|GripMotionControllerComponent|DropObjectbyInterface (Variables|/Script/VRExpansionPlugin.VRBaseCharacter|GetLeftMotionController (Utilities|Array|Get(acopy) _outactors)) 0 (.GripID (Utilities|Struct|BreakBPActorGripInformation _array_element)) "0, 0, 0" "0, 0, 0")
          (Audio|PlaySoundatLocation "/Game/VRE/Blueprints/Lantern/SFX/Flame.Flame" (Transformation|GetActorLocation) "0, 0, 0" 1.0 1.0 0.0 0 0 0 0)
          (Components|Activation|Activate (Variables|Default|GetP_Candle_Fire_Particle) false)
          (CallFunction|LanternFlight)))
      (:then_1
        (bind _griparray_2 (Class|GripMotionControllerComponent|GetAllGrips (Variables|/Script/VRExpansionPlugin.VRBaseCharacter|GetRightMotionController (Utilities|Array|Get(acopy) _outactors))))
        (for _array_element_2 _griparray_2
          (Class|GripMotionControllerComponent|DropObjectbyInterface (Variables|/Script/VRExpansionPlugin.VRBaseCharacter|GetRightMotionController (Utilities|Array|Get(acopy) _outactors)) 0 (.GripID (Utilities|Struct|BreakBPActorGripInformation _array_element_2)) "0, 0, 0" "0, 0, 0")
          (Audio|PlaySoundatLocation "/Game/VRE/Blueprints/Lantern/SFX/Flame.Flame" (Transformation|GetActorLocation) "0, 0, 0" 1.0 1.0 0.0 0 0 0 0)
          (Components|Activation|Activate (Variables|Default|GetP_Candle_Fire_Particle) false)
          (CallFunction|LanternFlight))))
    (else
      (Audio|PlaySound2D "/Game/VRE/Blueprints/Lantern/SFX/MatchStrikeDenied.MatchStrikeDenied" 1.0 1.0 0.0 0 0))))

(fn ConstructionScript)