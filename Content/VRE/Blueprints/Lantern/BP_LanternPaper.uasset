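; VR lantern paper piece that, when used while BP_LanternMain is Interacting, reveals the next paper-face stage of that lantern with a sound.
; A MultiGate starts from GateIndexMain stored on the lantern; the final stage changes material, flags the frame built and spawns BP_FlowerLantern.
; On grip release it destroys itself after a delay and spawns a replacement.
; DropAllItemsFunction empties both VR hands but is not called here.
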(event EventBeginPlay)

(event Collision|EventActorBeginOverlap
  (params (OtherActor :type Actor%20Object%20Reference)))

(event EventOnGripRelease
  (params (ReleasingController :type Grip%20Motion%20Controller%20Component%20Object%20Reference) (GripInformation :type BP%20Actor%20Grip%20Information%20Structure%20%28by%20ref%29) (bWasSocketed :type Boolean))
  (Utilities|FlowControl|Delay 1.0)
  (Actor|DestroyActor)
  (Game|SpawnActorfromClass "BP_LanternPaper_C" (Math|Transform|MakeTransform (Variables|Default|GetSpawn%20Transform%20Location%202) "90.000000,3870.000000,0.000000" (Variables|Default|GetSpawn%20Transform%20Scale)) "Undefined" "MultiplyWithRoot" 0 0))

(event EventOnUsed
  (bind _outactors (Actor|GetAllActorsOfClass "/Game/VRE/Blueprints/Lantern/BP_LanternMain.BP_LanternMain_C"))
  (Utilities|FlowControl|MultiGate false true (Variables|/Game/VRE/Blueprints/Lantern/BP_LanternMain.BP_LanternMain_C|GetGateIndexMain (Utilities|Array|Get(acopy) _outactors)) :!label _label
    (:Out%200
      (if (Variables|/Game/VRE/Blueprints/Lantern/BP_LanternMain.BP_LanternMain_C|Getinteracting (Utilities|Array|Get(acopy) _outactors))
        (Rendering|SetVisibility (Variables|/Game/VRE/Blueprints/Lantern/BP_LanternMain.BP_LanternMain_C|Get1__Lantern_-_Frame_with_1Face (Utilities|Array|Get(acopy) _outactors)) true false)
        (Audio|PlaySound2D "/Game/VRE/Blueprints/Lantern/SFX/PaperNoise.PaperNoise" 1.0 1.0 0.0 0 0)
        (Math|Integer|IncrementInt (Variables|/Game/VRE/Blueprints/Lantern/BP_LanternMain.BP_LanternMain_C|GetGateIndexMain (Utilities|Array|Get(acopy) _outactors)))
        (else
          (goto _label Reset))))
    (:Out%201
      (if (Variables|/Game/VRE/Blueprints/Lantern/BP_LanternMain.BP_LanternMain_C|Getinteracting (Utilities|Array|Get(acopy) _outactors))
        (Rendering|SetVisibility (Variables|/Game/VRE/Blueprints/Lantern/BP_LanternMain.BP_LanternMain_C|Get2__Lantern_-_Frame_with_2Faces (Utilities|Array|Get(acopy) _outactors)) true false)
        (Audio|PlaySound2D "/Game/VRE/Blueprints/Lantern/SFX/PaperNoise.PaperNoise" 1.0 1.0 0.0 0 0)
        (Math|Integer|IncrementInt (Variables|/Game/VRE/Blueprints/Lantern/BP_LanternMain.BP_LanternMain_C|GetGateIndexMain (Utilities|Array|Get(acopy) _outactors)))
        (else
          (goto _label Reset))))
    (:Out%202
      (if (Variables|/Game/VRE/Blueprints/Lantern/BP_LanternMain.BP_LanternMain_C|Getinteracting (Utilities|Array|Get(acopy) _outactors))
        (Rendering|SetVisibility (Variables|/Game/VRE/Blueprints/Lantern/BP_LanternMain.BP_LanternMain_C|Get3__Lantern_-_Frame_with_3Faces (Utilities|Array|Get(acopy) _outactors)) true false)
        (Audio|PlaySound2D "/Game/VRE/Blueprints/Lantern/SFX/PaperNoise.PaperNoise" 1.0 1.0 0.0 0 0)
        (Math|Integer|IncrementInt (Variables|/Game/VRE/Blueprints/Lantern/BP_LanternMain.BP_LanternMain_C|GetGateIndexMain (Utilities|Array|Get(acopy) _outactors)))
        (else
          (goto _label Reset))))
    (:Out%203
      (if (Variables|/Game/VRE/Blueprints/Lantern/BP_LanternMain.BP_LanternMain_C|Getinteracting (Utilities|Array|Get(acopy) _outactors))
        (Rendering|SetVisibility (Variables|/Game/VRE/Blueprints/Lantern/BP_LanternMain.BP_LanternMain_C|Get4__Lantern_-_Frame_with_4Faces (Utilities|Array|Get(acopy) _outactors)) true false)
        (Audio|PlaySound2D "/Game/VRE/Blueprints/Lantern/SFX/PaperNoise.PaperNoise" 1.0 1.0 0.0 0 0)
        (Math|Integer|IncrementInt (Variables|/Game/VRE/Blueprints/Lantern/BP_LanternMain.BP_LanternMain_C|GetGateIndexMain (Utilities|Array|Get(acopy) _outactors)))
        (else
          (goto _label Reset))))
    (:Out%204
      (if (Variables|/Game/VRE/Blueprints/Lantern/BP_LanternMain.BP_LanternMain_C|Getinteracting (Utilities|Array|Get(acopy) _outactors))
        (Rendering|SetVisibility (Variables|/Game/VRE/Blueprints/Lantern/BP_LanternMain.BP_LanternMain_C|Get5__Lantern_-_Frame_with_5Faces (Utilities|Array|Get(acopy) _outactors)) true false)
        (Audio|PlaySound2D "/Game/VRE/Blueprints/Lantern/SFX/PaperNoise.PaperNoise" 1.0 1.0 0.0 0 0)
        (Math|Integer|IncrementInt (Variables|/Game/VRE/Blueprints/Lantern/BP_LanternMain.BP_LanternMain_C|GetGateIndexMain (Utilities|Array|Get(acopy) _outactors)))
        (else
          (goto _label Reset))))
    (:Out%205
      (if (Variables|/Game/VRE/Blueprints/Lantern/BP_LanternMain.BP_LanternMain_C|Getinteracting (Utilities|Array|Get(acopy) _outactors))
        (Rendering|SetVisibility (Variables|/Game/VRE/Blueprints/Lantern/BP_LanternMain.BP_LanternMain_C|Get9__Lantern_-_with_3_golden_paper (Utilities|Array|Get(acopy) _outactors)) true false)
        (Audio|PlaySound2D "/Game/VRE/Blueprints/Lantern/SFX/PaperNoise.PaperNoise" 1.0 1.0 0.0 0 0)
        (Math|Integer|IncrementInt (Variables|/Game/VRE/Blueprints/Lantern/BP_LanternMain.BP_LanternMain_C|GetGateIndexMain (Utilities|Array|Get(acopy) _outactors))
          (:%20%20
            (Rendering|Material|SetMaterial (Variables|/Game/VRE/Blueprints/Lantern/BP_LanternMain.BP_LanternMain_C|Get9__Lantern_-_with_3_golden_paper (Utilities|Array|Get(acopy) _outactors)) 1 "/Game/StarterContent/Materials/M_Wood_Oak.M_Wood_Oak")
            (Audio|PlaySound2D "/Game/VRE/Blueprints/Lantern/SFX/Paper_Finish_Place.Paper_Finish_Place" 1.0 1.0 0.0 0 0)
            (Variables|/Game/VRE/Blueprints/Lantern/BP_LanternMain.BP_LanternMain_C|Setframe%20built%20main (Utilities|Array|Get(acopy) _outactors) true)
            (Game|SpawnActorfromClass "/Game/VRE/Blueprints/Lantern/BP_FlowerLantern.BP_FlowerLantern_C" (Math|Transform|MakeTransform (Variables|Default|GetFlower%20Spawn%20Loc) "180.000000,0.000000,0.000000" (Variables|Default|GetFlower%20Scale)) "Undefined" "MultiplyWithRoot" 0 0)))
        (else
          (goto _label Reset))))))

(fn ConstructionScript)

(fn DropAllItemsFunction
  (bind _outactors (Actor|GetAllActorsOfClass "/Game/VRE/Core/Character/BP_VRCharacter.BP_VRCharacter_C"))
  (Utilities|FlowControl|Sequence
    (:then_0
      (bind _griparray (Class|GripMotionControllerComponent|GetAllGrips (Variables|/Script/VRExpansionPlugin.VRBaseCharacter|GetLeftMotionController (Utilities|Array|Get(acopy) _outactors))))
      (for _array_element _griparray
        (Class|GripMotionControllerComponent|DropObjectbyInterface (Variables|/Script/VRExpansionPlugin.VRBaseCharacter|GetLeftMotionController (Utilities|Array|Get(acopy) _outactors)) 0 (.GripID (Utilities|Struct|BreakBPActorGripInformation _array_element)) "0, 0, 0" "0, 0, 0")))
    (:then_1
      (bind _griparray_2 (Class|GripMotionControllerComponent|GetAllGrips (Variables|/Script/VRExpansionPlugin.VRBaseCharacter|GetRightMotionController (Utilities|Array|Get(acopy) _outactors))))
      (for _array_element_2 _griparray_2
        (Class|GripMotionControllerComponent|DropObjectbyInterface (Variables|/Script/VRExpansionPlugin.VRBaseCharacter|GetRightMotionController (Utilities|Array|Get(acopy) _outactors)) 0 (.GripID (Utilities|Struct|BreakBPActorGripInformation _array_element_2)) "0, 0, 0" "0, 0, 0")))))