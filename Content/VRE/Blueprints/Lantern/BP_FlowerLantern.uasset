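; BP_FlowerLantern is a usable flower pickup that completes a lantern being built in the VRE lantern activity.
; On use it plays a pluck sound, then looks up the first BP_LanternMain in the level.
; If that lantern is being interacted with and its main frame is built, it reveals the flower-completed lantern component, flags the flower as built and destroys itself.
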(event EventBeginPlay)

(event Collision|EventActorBeginOverlap
  (params (OtherActor :type Actor%20Object%20Reference)))

(event EventOnUsed
  (Audio|PlaySound2D "/Game/VRE/Blueprints/Lantern/SFX/FlowerPluck.FlowerPluck" 1.0 1.0 0.0 0 0)
  (bind _outactors (Actor|GetAllActorsOfClass "/Game/VRE/Blueprints/Lantern/BP_LanternMain.BP_LanternMain_C"))
  (if (and (Variables|/Game/VRE/Blueprints/Lantern/BP_LanternMain.BP_LanternMain_C|Getinteracting (Utilities|Array|Get(acopy) _outactors)) (Variables|/Game/VRE/Blueprints/Lantern/BP_LanternMain.BP_LanternMain_C|Getframe%20built%20main (Utilities|Array|Get(acopy) _outactors)))
    (Rendering|SetVisibility (Variables|/Game/VRE/Blueprints/Lantern/BP_LanternMain.BP_LanternMain_C|Get14__Lantern_-_completed_with_flower (Utilities|Array|Get(acopy) _outactors)) true false)
    (Variables|/Game/VRE/Blueprints/Lantern/BP_LanternMain.BP_LanternMain_C|SetFlower%20Built (Utilities|Array|Get(acopy) _outactors) true)
    (Actor|DestroyActor)))

(fn ConstructionScript)