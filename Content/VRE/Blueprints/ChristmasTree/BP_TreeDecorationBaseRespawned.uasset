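; Grippable Christmas bauble for the VR tree-decorating activity, placed when used while its sphere overlaps BP_ChristmasTree.
; Placing plays a pop, increments the tree's bauble count and spawns a randomly coloured, query-only BP_TreeDecorationBase copy at the held position.
; Once the count reaches five, a per-instance DoOnce spawns BP_TreeStar.
; Releasing the grip destroys the actor after a short delay and spawns a BP_TreeDecorationBase at SpawnLocation.
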(event OnComponentBeginOverlap(Sphere)
  (params (OverlappedComponent :type Primitive%20Component%20Object%20Reference) (OtherActor :type Actor%20Object%20Reference) (OtherComp :type Primitive%20Component%20Object%20Reference) (OtherBodyIndex :type Integer) (bFromSweep :type Boolean) (SweepResult :type Hit%20Result%20Structure%20%28by%20ref%29))
  (Utilities|Casting|CastToBP_ChristmasTree OtherActor)
  (Variables|Default|SetInteracting true))

(event OnComponentEndOverlap(Sphere)
  (params (OverlappedComponent :type Primitive%20Component%20Object%20Reference) (OtherActor :type Actor%20Object%20Reference) (OtherComp :type Primitive%20Component%20Object%20Reference) (OtherBodyIndex :type Integer))
  (Utilities|Casting|CastToBP_ChristmasTree OtherActor)
  (Variables|Default|SetInteracting false))

(event Custom|PlaceDecoration
  (bind _staticmeshcomponent (Variables|Default|GetStaticMeshComponent))
  (bind _outactors (Actor|GetAllActorsOfClass "/Game/VRE/Blueprints/ChristmasTree/BP_ChristmasTree.BP_ChristmasTree_C"))
  (bind _result (Math|Integer|IncrementInt (Variables|/Game/VRE/Blueprints/ChristmasTree/BP_ChristmasTree.BP_ChristmasTree_C|Getamount%20baubles%20placed (Utilities|Array|Get(acopy) _outactors)))
    (:%20%20
      (bind _returnvalue (Game|SpawnActorfromClass "/Game/VRE/Blueprints/ChristmasTree/BP_TreeDecorationBase.BP_TreeDecorationBase_C" (Math|Transform|MakeTransform (Transformation|GetWorldLocation _staticmeshcomponent) (Transformation|GetWorldRotation _staticmeshcomponent) "1.000000,1.000000,1.000000") "Undefined" "MultiplyWithRoot" 0 0))
      (Collision|SetCollisionEnabled (Variables|/Script/Engine.StaticMeshActor|GetStaticMeshComponent _returnvalue) "QueryOnly")
      (switch int (Math|Random|RandomInteger 4)
        (:0
          (Rendering|Material|SetMaterial (Variables|/Script/Engine.StaticMeshActor|GetStaticMeshComponent _returnvalue) 0 (Variables|Default|GetM_Green)))
        (:1
          (Rendering|Material|SetMaterial (Variables|/Script/Engine.StaticMeshActor|GetStaticMeshComponent _returnvalue) 0 (Variables|Default|GetM_Gold)))
        (:2
          (Rendering|Material|SetMaterial (Variables|/Script/Engine.StaticMeshActor|GetStaticMeshComponent _returnvalue) 0 (Variables|Default|GetM_Pink)))
        (:3
          (Rendering|Material|SetMaterial (Variables|/Script/Engine.StaticMeshActor|GetStaticMeshComponent _returnvalue) 0 (Variables|Default|GetM_Blue)))
        (:4
          (Rendering|Material|SetMaterial (Variables|/Script/Engine.StaticMeshActor|GetStaticMeshComponent _returnvalue) 0 (Variables|Default|GetM_Red)))))))

(event Custom|SpawnStar
  ;[1 1 1] Spawn Star at location in the world (Add Logic)
  (Game|SpawnActorfromClass "/Game/VRE/Blueprints/ChristmasTree/BP_TreeStar.BP_TreeStar_C" (Math|Transform|MakeTransform (Variables|Default|GetSpawn%20Location_0) "0, 0, 0" "1.000000,1.000000,1.000000") "Undefined" "MultiplyWithRoot" 0 0))

(event EventOnGripRelease
  (params (ReleasingController :type Grip%20Motion%20Controller%20Component%20Object%20Reference) (GripInformation :type BP%20Actor%20Grip%20Information%20Structure%20%28by%20ref%29) (bWasSocketed :type Boolean))
  (Utilities|FlowControl|Delay 1.0)
  (Actor|DestroyActor)
  (Game|SpawnActorfromClass "/Game/VRE/Blueprints/ChristmasTree/BP_TreeDecorationBase.BP_TreeDecorationBase_C" (Math|Transform|MakeTransform (Variables|Default|GetSpawn%20Location) "0, 0, 0" "1.000000,1.000000,1.000000") "Undefined" "MultiplyWithRoot" 0 0))

(event EventOnUsed
  (if (Variables|Default|GetInteracting)
    (Audio|PlaySound2D "/Game/VRE/Blueprints/ChristmasTree/PopSound.PopSound" 1.0 1.0 0.0 0 0)
    (CallFunction|PlaceDecoration)
    (if (>= (stale Custom|PlaceDecoration _result) 5)
      (Variables|Default|SetCanPlaceStar true)
      (Utilities|FlowControl|DoOnce false
        (:Completed
          (CallFunction|SpawnStar)))
      (else
        (Variables|Default|SetCanPlaceStar false)))))

(fn ConstructionScript)