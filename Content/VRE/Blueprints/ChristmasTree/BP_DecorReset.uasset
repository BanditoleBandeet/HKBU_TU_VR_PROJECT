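; BP_DecorReset is a button actor that clears the Christmas tree decorations.
; On any button state change it destroys every BP_TreeDecorationBase actor, then every BP_TreeStar.
; It fires the TreeRest dispatcher inside the decoration loop, so reset listeners are notified once per destroyed decoration and not at all when none exist.
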(event OnButtonStateChanged(ButtonComp)
  (params (ButtonState :type Boolean) (InteractingActor :type Actor%20Object%20Reference) (InteractingComponent :type Primitive%20Component%20Object%20Reference))
  ;[1 1 1] Deletes all actors of the class and sends out a dispatcher message to be called in the reset logic
  (Utilities|FlowControl|Sequence
    (:then_0
      (bind _outactors (Actor|GetAllActorsOfClass "/Game/VRE/Blueprints/ChristmasTree/BP_TreeDecorationBase.BP_TreeDecorationBase_C"))
      (for _array_element _outactors
        (Actor|DestroyActor _array_element)
        (Default|CallTreeRest)))
    (:then_1
      (bind _outactors_2 (Actor|GetAllActorsOfClass "/Game/VRE/Blueprints/ChristmasTree/BP_TreeStar.BP_TreeStar_C"))
      (for _array_element_2 _outactors_2
        (Actor|DestroyActor _array_element_2)))))

(event EventBeginPlay
  (|CallParentFunction) ; This node is disabled and will not be called.\nDrag off pins to build functionality.
)

(event Collision|EventActorBeginOverlap
  (params (OtherActor :type Actor%20Object%20Reference)))

(fn ConstructionScript
  (|CallParentFunction))