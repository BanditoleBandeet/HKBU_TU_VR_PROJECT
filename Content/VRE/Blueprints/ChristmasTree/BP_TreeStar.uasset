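; BP_TreeStar is a usable star that can be placed on the Christmas tree in the VRE content.
; Its box overlap tracks whether it is touching a BP_ChristmasTree through an Interacting flag.
; Using it while touching the tree plays a pop sound and spawns a collision-free copy at the mesh's location and rotation.
; The original star is not destroyed or detached.
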(event OnComponentBeginOverlap(Box)
  (params (OverlappedComponent :type Primitive%20Component%20Object%20Reference) (OtherActor :type Actor%20Object%20Reference) (OtherComp :type Primitive%20Component%20Object%20Reference) (OtherBodyIndex :type Integer) (bFromSweep :type Boolean) (SweepResult :type Hit%20Result%20Structure%20%28by%20ref%29))
  (Utilities|Casting|CastToBP_ChristmasTree OtherActor)
  (Variables|Default|SetInteracting true))

(event OnComponentEndOverlap(Box)
  (params (OverlappedComponent :type Primitive%20Component%20Object%20Reference) (OtherActor :type Actor%20Object%20Reference) (OtherComp :type Primitive%20Component%20Object%20Reference) (OtherBodyIndex :type Integer))
  (Utilities|Casting|CastToBP_ChristmasTree OtherActor)
  (Variables|Default|SetInteracting false))

(event Custom|Place%20Star
  (bind _staticmeshcomponent (Variables|Default|GetStaticMeshComponent))
  (bind _returnvalue (Game|SpawnActorfromClass "BP_TreeStar_C" (Math|Transform|MakeTransform (Transformation|GetWorldLocation _staticmeshcomponent) (Transformation|GetWorldRotation _staticmeshcomponent) "1.000000,1.000000,1.000000") "Undefined" "MultiplyWithRoot" 0 0))
  (Collision|SetCollisionEnabled (Variables|/Script/Engine.StaticMeshActor|GetStaticMeshComponent _returnvalue) "NoCollision"))

(event EventOnUsed
  (if (Variables|Default|GetInteracting)
    (Audio|PlaySound2D "/Game/VRE/Blueprints/ChristmasTree/PopSound.PopSound" 1.0 1.0 0.0 0 0)
    (CallFunction|PlaceStar)))

(fn ConstructionScript)