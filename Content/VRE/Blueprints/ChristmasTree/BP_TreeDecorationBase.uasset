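; Base actor for a Christmas tree decoration that leaves a copy of itself on the tree when used.
; A sphere overlap with BP_ChristmasTree gates OnUsed, which spawns a new decoration at the mesh's location and rotation.
; Each copy gets query-only collision and a random material, and the placed count increments.
; From the fifth placement onward, each use also enables star placement and spawns a BP_TreeStar.
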(event OnComponentBeginOverlap(Sphere)
  (params (OverlappedComponent :type Primitive%20Component%20Object%20Reference) (OtherActor :type Actor%20Object%20Reference) (OtherComp :type Primitive%20Component%20Object%20Reference) (OtherBodyIndex :type Integer) (bFromSweep :type Boolean) (SweepResult :type Hit%20Result%20Structure%20%28by%20ref%29))
  (Utilities|Casting|CastToBP_ChristmasTree OtherActor)
  (Variables|Default|SetInteracting true))

(event OnComponentEndOverlap(Sphere)
  (params (OverlappedComponent :type Primitive%20Component%20Object%20Reference) (OtherActor :type Actor%20Object%20Reference) (OtherComp :type Primitive%20Component%20Object%20Reference) (OtherBodyIndex :type Integer))
  (Utilities|Casting|CastToBP_ChristmasTree OtherActor)
  (Variables|Default|SetInteracting false))

(event Custom|PlaceDecoration
  (bind _staticmeshcomponent (Variables|Default|GetStaticMeshComponent))
  (bind _result (Math|Integer|IncrementInt (Variables|Default|GetAmountPlaced))
    (:%20%20
      (bind _returnvalue (Game|SpawnActorfromClass "BP_TreeDecorationBase_C" (Math|Transform|MakeTransform (Transformation|GetWorldLocation _staticmeshcomponent) (Transformation|GetWorldRotation _staticmeshcomponent) "1.000000,1.000000,1.000000") "Undefined" "MultiplyWithRoot" 0 0))
      (Collision|SetCollisionEnabled (Variables|/Script/Engine.StaticMeshActor|GetStaticMeshComponent _returnvalue) "QueryOnly")
      (switch int (Math|Random|RandomInteger 5)
        (:0
          (Rendering|Material|SetMaterial (Variables|/Script/Engine.StaticMeshActor|GetStaticMeshComponent _returnvalue) 0 (Variables|Default|GetM_RED)))
        (:1
          (Rendering|Material|SetMaterial (Variables|/Script/Engine.StaticMeshActor|GetStaticMeshComponent _returnvalue) 0 (Variables|Default|GetM_YELLOW)))
        (:2
          (Rendering|Material|SetMaterial (Variables|/Script/Engine.StaticMeshActor|GetStaticMeshComponent _returnvalue) 0 (Variables|Default|GetM_TBD1)))
        (:3
          (Rendering|Material|SetMaterial (Variables|/Script/Engine.StaticMeshActor|GetStaticMeshComponent _returnvalue) 0 (Variables|Default|GetM_TBD2)))
        (:4
          (Rendering|Material|SetMaterial (Variables|/Script/Engine.StaticMeshActor|GetStaticMeshComponent _returnvalue) 0 (Variables|Default|GetM_TBD3)))))))

(event Custom|SpawnStar
  ;[1 1 1] Spawn Star at location in the world (Add Logic)
  (Game|SpawnActorfromClass "/Game/VRE/Blueprints/ChristmasTree/BP_TreeStar.BP_TreeStar_C" (Math|Transform|MakeTransform (Variables|Default|GetSpawn%20Location) "0, 0, 0" "1.000000,1.000000,1.000000") "Undefined" "MultiplyWithRoot" 0 0))

(event EventOnUsed
  (if (Variables|Default|GetInteracting)
    (CallFunction|PlaceDecoration)
    (if (>= (stale Custom|PlaceDecoration _result) 5)
      (Variables|Default|SetCanPlaceStar true)
      (CallFunction|SpawnStar)
      (else
        (Variables|Default|SetCanPlaceStar false)))))

(fn ConstructionScript)