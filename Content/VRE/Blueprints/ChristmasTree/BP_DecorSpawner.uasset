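; Button-driven spawner that creates a tree decoration for the Christmas tree scene.
; A state change on its button component spawns a BP_TreeDecorationBase at SpawnLocation, gated by a DoOnce so it fires only once.
; Each state change also binds to the first BP_DecorReset found in the level, whose tree reset event re-arms the DoOnce.
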(event OnButtonStateChanged(ButtonComp)
  (params (ButtonState :type Boolean) (InteractingActor :type Actor%20Object%20Reference) (InteractingComponent :type Primitive%20Component%20Object%20Reference))
  ;[1 1 1] on button state change, spawn spawn the decoration actor at location. will spawn once and then reet the do once if the tree has been reset
  (bind _outactors (Actor|GetAllActorsOfClass "/Game/VRE/Blueprints/ChristmasTree/BP_DecorReset.BP_DecorReset_C"))
  (EventDispatchers|BindEventtoTreeRest (Utilities|Array|Get(acopy) _outactors) (delegate Custom|Tree%20Reset%20Check))
  (Utilities|FlowControl|DoOnce false
    (:Completed
      (Game|SpawnActorfromClass "/Game/VRE/Blueprints/ChristmasTree/BP_TreeDecorationBase.BP_TreeDecorationBase_C" (Math|Transform|MakeTransform (Variables|Default|Getspawn%20location) "0, 0, 0" "1.000000,1.000000,1.000000") "Undefined" "MultiplyWithRoot" 0 0))))

(event Custom|Tree%20Reset%20Check
  ;[1 1 1] on button state change, spawn spawn the decoration actor at location. will spawn once and then reet the do once if the tree has been reset
  (Utilities|FlowControl|DoOnce false) ; enters at Reset
)

(event EventBeginPlay
  (|CallParentFunction) ; This node is disabled and will not be called.\nDrag off pins to build functionality.
)

(event Collision|EventActorBeginOverlap
  (params (OtherActor :type Actor%20Object%20Reference)))

(fn ConstructionScript
  (|CallParentFunction))