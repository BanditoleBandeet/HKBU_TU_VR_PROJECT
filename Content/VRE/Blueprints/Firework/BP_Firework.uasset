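; Grippable VR firework that lights its fuse when used, then launches on grip release if lit.
; A timeline update pushes the actor along its arrow by a fixed step per tick, so speed depends on frame rate.
; A delay and DoOnce fed from that update trigger one burst with audio and one of five random VFX.
; The burst hides the mesh, stops the fuse effects and later deactivates all firework VFX.
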(event Custom|FireworkEvent
  (Components|Timeline|SetPlayRate (Variables|Default|GetTimeline) (/ 1.0 (Variables|Default|Gettimeline%20length)))
  (Timeline|Timeline PlayFromStart
    (:Update
      (Transformation|SetActorLocation (+ (Transformation|GetActorLocation) (* (Math|Vector|GetForwardVector (Variables|Default|GetArrow)) 3e+01)) false false)
      (Utilities|FlowControl|Delay 2.0)
      (Utilities|FlowControl|DoOnce false
        (:Completed
          (Audio|Components|Audio|Play (Variables|Default|GetAudio) 0.0)
          (switch int (Math|Random|RandomInteger 5)
            (:0
              (Components|Activation|Activate (Variables|Default|GetVFX%20Firework) false))
            (:1
              (Components|Activation|Activate (Variables|Default|GetVFX%20Firework1) false))
            (:2
              (Components|Activation|Activate (Variables|Default|GetVFX%20Firework2) false))
            (:3
              (Components|Activation|Activate (Variables|Default|GetVFX%20Firework3) false))
            (:4
              (Components|Activation|Activate (Variables|Default|GetVFX%20Firework4) false)))
          (Rendering|SetVisibility (Variables|Default|GetStaticMeshComponent) false false)
          (Components|Activation|Deactivate (Variables|Default|GetP_Sparks))
          (Audio|Components|Audio|Stop (Variables|Default|GetFuzeLitAudio))
          (Utilities|FlowControl|Delay 3.5)
          (Components|Activation|Deactivate (Variables|Default|GetVFX%20Firework)))))))

(event EventOnUsed
  (Variables|Default|SetHasClicked true)
  (Components|Activation|Activate (Variables|Default|GetP_Sparks) false)
  (Audio|Components|Audio|Play (Variables|Default|GetFuzeLitAudio) 0.0))

(event EventOnGripRelease
  (params (ReleasingController :type Grip%20Motion%20Controller%20Component%20Object%20Reference) (GripInformation :type BP%20Actor%20Grip%20Information%20Structure%20%28by%20ref%29) (bWasSocketed :type Boolean))
  (if (Variables|Default|GetHasClicked)
    (CallFunction|FireworkEvent)))

(fn ConstructionScript)