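; An inventory slot collision component for VR that snaps a released inventory item onto itself.
; On overlap it stores one BP_InventoryActor held by a motion controller, skipping items held by the optional ControllerToIgnore.
; Ending that actor's overlap clears the stored reference.
; Tick attaches the stored actor to the component whenever it has no valid controller, snapping location and rotation while keeping world scale.
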(event Custom|Begin_Overlap
  (params (OverlappedComponent :type Primitive%20Component%20Object%20Reference) (OtherActor :type Actor%20Object%20Reference) (OtherComp :type Primitive%20Component%20Object%20Reference) (OtherBodyIndex :type Integer) (bFromSweep :type Boolean) (SweepResult :type Hit%20Result%20Structure%20%28by%20ref%29))
  (bind _controllertoignore (Variables|Default|GetControllerToIgnore))
  (Utilities|IsValid (Variables|Default|GetGrabActor)
    (:Is%20Not%20Valid
      ;[1 1 1] Checks if you are dealing with a inventory actor or a child of inventory actor parent
      (bind _asbp_inventory_actor (Utilities|Casting|CastToBP_InventoryActor OtherActor))
      (Utilities|IsValid (Variables|/Game/VRE/Blueprints/Inventory/BP_InventoryActor.BP_InventoryActor_C|GetMotion%20Controller _asbp_inventory_actor)
        (:Is%20Valid
          (Utilities|IsValid _controllertoignore
            (:Is%20Valid
              (if (!= _controllertoignore (Variables|/Game/VRE/Blueprints/Inventory/BP_InventoryActor.BP_InventoryActor_C|GetMotion%20Controller _asbp_inventory_actor))
                (Variables|Default|SetGrabActor _asbp_inventory_actor :!label _label)))
            (:Is%20Not%20Valid
              (goto _label))))))))

(event Custom|End_Overlap
  (params (OverlappedComponent :type Primitive%20Component%20Object%20Reference) (OtherActor :type Actor%20Object%20Reference) (OtherComp :type Primitive%20Component%20Object%20Reference) (OtherBodyIndex :type Integer))
  (if (== (Variables|Default|GetGrabActor) OtherActor)
    (Variables|Default|SetGrabActor 0)))

(event EventBeginPlay
  (Collision|BindEventtoOnComponentBeginOverlap (delegate Custom|Begin_Overlap))
  (Collision|BindEventtoOnComponentEndOverlap (delegate Custom|End_Overlap)))

(event EventTick
  (params (DeltaSeconds :type Float%20%28single-precision%29))
  (bind _grabactor (Variables|Default|GetGrabActor))
  ;[1 1 1] Checking item is in range to be grabbed
  (Utilities|IsValid _grabactor
    (:Is%20Valid
      (Utilities|IsValid (Variables|/Game/VRE/Blueprints/Inventory/BP_InventoryActor.BP_InventoryActor_C|GetMotion%20Controller _grabactor)
        (:Is%20Not%20Valid
          (Transformation|AttachComponentToComponent _grabactor self "None" "SnapToTarget" "SnapToTarget" "KeepWorld" true))))))