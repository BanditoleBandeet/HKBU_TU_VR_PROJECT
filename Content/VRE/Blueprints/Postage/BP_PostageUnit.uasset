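; VR postage sorting unit with red, blue, yellow and green boxes that each react to a postage item of the matching colour.
; On overlap, a box sets its Interacting flag and force-drops every grip on both motion controllers of the first BP_VRCharacter.
; Only red then disables gravity on the first red item found and moves it to RedPoint.
; Blue's move is disconnected, while yellow and green only look up their items.
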(event OnComponentBeginOverlap(redbox)
  (params (OverlappedComponent :type Primitive%20Component%20Object%20Reference) (OtherActor :type Actor%20Object%20Reference) (OtherComp :type Primitive%20Component%20Object%20Reference) (OtherBodyIndex :type Integer) (bFromSweep :type Boolean) (SweepResult :type Hit%20Result%20Structure%20%28by%20ref%29))
  (Utilities|Casting|CastToBP_PostageItem_Red OtherActor)
  (Variables|Default|SetRedInteracting true)
  (bind _outactors (Actor|GetAllActorsOfClass "/Game/VRE/Core/Character/BP_VRCharacter.BP_VRCharacter_C"))
  (Utilities|FlowControl|Sequence
    (:then_0
      (bind _griparray (Class|GripMotionControllerComponent|GetAllGrips (Variables|/Script/VRExpansionPlugin.VRBaseCharacter|GetLeftMotionController (Utilities|Array|Get(acopy) _outactors))))
      (for _array_element _griparray
        (Class|GripMotionControllerComponent|DropObjectbyInterface (Variables|/Script/VRExpansionPlugin.VRBaseCharacter|GetLeftMotionController (Utilities|Array|Get(acopy) _outactors)) 0 (.GripID (Utilities|Struct|BreakBPActorGripInformation _array_element)) "0, 0, 0" "0, 0, 0")
        (bind _outactors_2 (Actor|GetAllActorsOfClass "/Game/VRE/Blueprints/Postage/BP_PostageItem_Red.BP_PostageItem_Red_C"))
        (Physics|SetEnableGravity (Variables|/Script/Engine.StaticMeshActor|GetStaticMeshComponent (Utilities|Array|Get(acopy) _outactors_2)) false)
        (Transformation|SetWorldLocation (Variables|/Script/Engine.StaticMeshActor|GetStaticMeshComponent (Utilities|Array|Get(acopy) _outactors_2)) (Transformation|GetWorldLocation (Variables|Default|Getred%20point)) false false)))
    (:then_1
      (bind _griparray_2 (Class|GripMotionControllerComponent|GetAllGrips (Variables|/Script/VRExpansionPlugin.VRBaseCharacter|GetRightMotionController (Utilities|Array|Get(acopy) _outactors))))
      (for _array_element_2 _griparray_2
        (Class|GripMotionControllerComponent|DropObjectbyInterface (Variables|/Script/VRExpansionPlugin.VRBaseCharacter|GetRightMotionController (Utilities|Array|Get(acopy) _outactors)) 0 (.GripID (Utilities|Struct|BreakBPActorGripInformation _array_element_2)) "0, 0, 0" "0, 0, 0")
        (bind _outactors_3 (Actor|GetAllActorsOfClass "/Game/VRE/Blueprints/Postage/BP_PostageItem_Red.BP_PostageItem_Red_C"))
        (Physics|SetEnableGravity (Variables|/Script/Engine.StaticMeshActor|GetStaticMeshComponent (Utilities|Array|Get(acopy) _outactors_3)) false)
        (Transformation|SetWorldLocation (Variables|/Script/Engine.StaticMeshActor|GetStaticMeshComponent (Utilities|Array|Get(acopy) _outactors_3)) (Transformation|GetWorldLocation (Variables|Default|Getred%20point)) false false)))))

(event OnComponentBeginOverlap(bluebox)
  (params (OverlappedComponent :type Primitive%20Component%20Object%20Reference) (OtherActor :type Actor%20Object%20Reference) (OtherComp :type Primitive%20Component%20Object%20Reference) (OtherBodyIndex :type Integer) (bFromSweep :type Boolean) (SweepResult :type Hit%20Result%20Structure%20%28by%20ref%29))
  (Utilities|Casting|CastToBP_PostageItem_Blue OtherActor)
  (Variables|Default|SetBlueInteracting true)
  (bind _outactors (Actor|GetAllActorsOfClass "/Game/VRE/Core/Character/BP_VRCharacter.BP_VRCharacter_C"))
  (Utilities|FlowControl|Sequence
    (:then_0
      (bind _griparray (Class|GripMotionControllerComponent|GetAllGrips (Variables|/Script/VRExpansionPlugin.VRBaseCharacter|GetLeftMotionController (Utilities|Array|Get(acopy) _outactors))))
      (for _array_element _griparray
        (Class|GripMotionControllerComponent|DropObjectbyInterface (Variables|/Script/VRExpansionPlugin.VRBaseCharacter|GetLeftMotionController (Utilities|Array|Get(acopy) _outactors)) 0 (.GripID (Utilities|Struct|BreakBPActorGripInformation _array_element)) "0, 0, 0" "0, 0, 0")
        (bind _outactors_2 (Actor|GetAllActorsOfClass "/Game/VRE/Blueprints/Postage/BP_PostageItem_Blue.BP_PostageItem_Blue_C"))))
    (:then_1
      (bind _griparray_2 (Class|GripMotionControllerComponent|GetAllGrips (Variables|/Script/VRExpansionPlugin.VRBaseCharacter|GetRightMotionController (Utilities|Array|Get(acopy) _outactors))))
      (for _array_element_2 _griparray_2
        (Class|GripMotionControllerComponent|DropObjectbyInterface (Variables|/Script/VRExpansionPlugin.VRBaseCharacter|GetRightMotionController (Utilities|Array|Get(acopy) _outactors)) 0 (.GripID (Utilities|Struct|BreakBPActorGripInformation _array_element_2)) "0, 0, 0" "0, 0, 0")
        (bind _outactors_3 (Actor|GetAllActorsOfClass "/Game/VRE/Blueprints/Postage/BP_PostageItem_Blue.BP_PostageItem_Blue_C"))))))

(event OnComponentBeginOverlap(yellowbox)
  (params (OverlappedComponent :type Primitive%20Component%20Object%20Reference) (OtherActor :type Actor%20Object%20Reference) (OtherComp :type Primitive%20Component%20Object%20Reference) (OtherBodyIndex :type Integer) (bFromSweep :type Boolean) (SweepResult :type Hit%20Result%20Structure%20%28by%20ref%29))
  (Utilities|Casting|CastToBP_PostageItem_Yellow OtherActor)
  (Variables|Default|SetYellowInteracting true)
  (bind _outactors (Actor|GetAllActorsOfClass "/Game/VRE/Core/Character/BP_VRCharacter.BP_VRCharacter_C"))
  (Utilities|FlowControl|Sequence
    (:then_0
      (bind _griparray (Class|GripMotionControllerComponent|GetAllGrips (Variables|/Script/VRExpansionPlugin.VRBaseCharacter|GetLeftMotionController (Utilities|Array|Get(acopy) _outactors))))
      (for _array_element _griparray
        (Class|GripMotionControllerComponent|DropObjectbyInterface (Variables|/Script/VRExpansionPlugin.VRBaseCharacter|GetLeftMotionController (Utilities|Array|Get(acopy) _outactors)) 0 (.GripID (Utilities|Struct|BreakBPActorGripInformation _array_element)) "0, 0, 0" "0, 0, 0")
        (Actor|GetAllActorsOfClass "/Game/VRE/Blueprints/Postage/BP_PostageItem_Yellow.BP_PostageItem_Yellow_C")))
    (:then_1
      (bind _griparray_2 (Class|GripMotionControllerComponent|GetAllGrips (Variables|/Script/VRExpansionPlugin.VRBaseCharacter|GetRightMotionController (Utilities|Array|Get(acopy) _outactors))))
      (for _array_element_2 _griparray_2
        (Class|GripMotionControllerComponent|DropObjectbyInterface (Variables|/Script/VRExpansionPlugin.VRBaseCharacter|GetRightMotionController (Utilities|Array|Get(acopy) _outactors)) 0 (.GripID (Utilities|Struct|BreakBPActorGripInformation _array_element_2)) "0, 0, 0" "0, 0, 0")
        (Actor|GetAllActorsOfClass "/Game/VRE/Blueprints/Postage/BP_PostageItem_Yellow.BP_PostageItem_Yellow_C")))))

(event OnComponentBeginOverlap(greenbox)
  (params (OverlappedComponent :type Primitive%20Component%20Object%20Reference) (OtherActor :type Actor%20Object%20Reference) (OtherComp :type Primitive%20Component%20Object%20Reference) (OtherBodyIndex :type Integer) (bFromSweep :type Boolean) (SweepResult :type Hit%20Result%20Structure%20%28by%20ref%29))
  (Utilities|Casting|CastToBP_PostageItem_Green OtherActor)
  (Variables|Default|SetGreenInteracting true)
  (bind _outactors (Actor|GetAllActorsOfClass "/Game/VRE/Core/Character/BP_VRCharacter.BP_VRCharacter_C"))
  (Utilities|FlowControl|Sequence
    (:then_0
      (bind _griparray (Class|GripMotionControllerComponent|GetAllGrips (Variables|/Script/VRExpansionPlugin.VRBaseCharacter|GetLeftMotionController (Utilities|Array|Get(acopy) _outactors))))
      (for _array_element _griparray
        (Class|GripMotionControllerComponent|DropObjectbyInterface (Variables|/Script/VRExpansionPlugin.VRBaseCharacter|GetLeftMotionController (Utilities|Array|Get(acopy) _outactors)) 0 (.GripID (Utilities|Struct|BreakBPActorGripInformation _array_element)) "0, 0, 0" "0, 0, 0")
        (Actor|GetAllActorsOfClass "/Game/VRE/Blueprints/Postage/BP_PostageItem_Green.BP_PostageItem_Green_C")))
    (:then_1
      (bind _griparray_2 (Class|GripMotionControllerComponent|GetAllGrips (Variables|/Script/VRExpansionPlugin.VRBaseCharacter|GetRightMotionController (Utilities|Array|Get(acopy) _outactors))))
      (for _array_element_2 _griparray_2
        (Class|GripMotionControllerComponent|DropObjectbyInterface (Variables|/Script/VRExpansionPlugin.VRBaseCharacter|GetRightMotionController (Utilities|Array|Get(acopy) _outactors)) 0 (.GripID (Utilities|Struct|BreakBPActorGripInformation _array_element_2)) "0, 0, 0" "0, 0, 0")
        (Actor|GetAllActorsOfClass "/Game/VRE/Blueprints/Postage/BP_PostageItem_Green.BP_PostageItem_Green_C")))))

(fn ConstructionScript)