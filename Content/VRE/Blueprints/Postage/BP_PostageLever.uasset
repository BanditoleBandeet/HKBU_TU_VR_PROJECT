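; BP_PostageLever is a VR lever that makes BP_Cabinet1 spawn a random burst of red, blue, green or yellow items.
; Tick polls the lever angle and, past a threshold, force-drops everything held by the VR character's motion controllers.
; Each drop starts a looping timer that calls a random color spawn on the cabinet.
; The timer event clears that timer after a short, partly randomized delay, limiting the burst.
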(event Custom|Spawn%20Multiple
  (switch int (Math|Random|RandomIntegerinRange 0 3)
    (:0
      (Default|SpawnRed (Utilities|Array|Get(acopy) (stale EventTick _outactors_3))))
    (:1
      (Default|SpawnBlue (Utilities|Array|Get(acopy) (stale EventTick _outactors_3))))
    (:2
      (Default|SpawnGreen (Utilities|Array|Get(acopy) (stale EventTick _outactors_3))))
    (:3
      (Default|SpawnYellow (Utilities|Array|Get(acopy) (stale EventTick _outactors_3))))))

(event Custom|CustomEvent
  (bind _returnvalue (Math|Random|RandomFloatinRange 0.0 2.0))
  (CallFunction|SpawnMultiple)
  (if (< _returnvalue 0.5)
    (bind _output_get (Variables|Default|SetTimer 0.5))
    (Utilities|FlowControl|Delay _output_get)
    (Utilities|Time|ClearandInvalidateTimerbyHandle (stale EventTick _returnvalue_2))
    (else
      (Utilities|FlowControl|Delay _returnvalue)
      (Utilities|Time|ClearandInvalidateTimerbyHandle (stale EventTick _returnvalue_2)))))

(event Collision|EventActorBeginOverlap
  (params (OtherActor :type Actor%20Object%20Reference))
  (|CallParentFunction OtherActor) ; This node is disabled and will not be called.\nDrag off pins to build functionality.
)

(event EventTick
  (params (DeltaSeconds :type Float%20%28single-precision%29))
  (|CallParentFunction DeltaSeconds)
  (if (<= (Variables|/Script/VRExpansionPlugin.VRLeverComponent|GetCurrentLeverAngle (Variables|Default|GetVRLever)) -3e+01)
    (bind _outactors (Actor|GetAllActorsOfClass "/Game/VRE/Core/Character/BP_VRCharacter.BP_VRCharacter_C"))
    (Utilities|FlowControl|Sequence
      (:then_0
        (bind _griparray (Class|GripMotionControllerComponent|GetAllGrips (Variables|/Script/VRExpansionPlugin.VRBaseCharacter|GetLeftMotionController (Utilities|Array|Get(acopy) _outactors))))
        (for _array_element _griparray
          (Class|GripMotionControllerComponent|DropObjectbyInterface (Variables|/Script/VRExpansionPlugin.VRBaseCharacter|GetLeftMotionController (Utilities|Array|Get(acopy) _outactors)) 0 (.GripID (Utilities|Struct|BreakBPActorGripInformation _array_element)) "0, 0, 0" "0, 0, 0")
          (bind _outactors_2 (Actor|GetAllActorsOfClass "/Game/VRE/Blueprints/Postage/BP_Cabinet1.BP_Cabinet1_C"))
          (bind _returnvalue (Utilities|Time|SetTimerbyEvent (delegate Custom|CustomEvent) 0.5 true))))
      (:then_1
        (bind _griparray_2 (Class|GripMotionControllerComponent|GetAllGrips (Variables|/Script/VRExpansionPlugin.VRBaseCharacter|GetRightMotionController (Utilities|Array|Get(acopy) _outactors))))
        (for _array_element_2 _griparray_2
          (Class|GripMotionControllerComponent|DropObjectbyInterface (Variables|/Script/VRExpansionPlugin.VRBaseCharacter|GetRightMotionController (Utilities|Array|Get(acopy) _outactors)) 0 (.GripID (Utilities|Struct|BreakBPActorGripInformation _array_element_2)) "0, 0, 0" "0, 0, 0")
          (bind _outactors_3 (Actor|GetAllActorsOfClass "/Game/VRE/Blueprints/Postage/BP_Cabinet1.BP_Cabinet1_C"))
          (bind _returnvalue_2 (Utilities|Time|SetTimerbyEvent (delegate Custom|CustomEvent) 0.5 true)))))))

(fn ConstructionScript
  (|CallParentFunction))