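; BP_Cabinet1 is a cabinet that tracks whether its red and blue doors are closed and spawns colored postage items.
; Door sphere overlap events re-test each door sphere against its paired sphere to set RedClosed and BlueClosed.
; Four custom events spawn red, blue, yellow or green items at their billboard markers.
; Nothing in this graph triggers those spawns, as the chain calling them is disconnected.
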(event OnComponentBeginOverlap(SphereDoor4)
  (params (OverlappedComponent :type Primitive%20Component%20Object%20Reference) (OtherActor :type Actor%20Object%20Reference) (OtherComp :type Primitive%20Component%20Object%20Reference) (OtherBodyIndex :type Integer) (bFromSweep :type Boolean) (SweepResult :type Hit%20Result%20Structure%20%28by%20ref%29))
  ;[1 1 1] Red Door Check
  (Variables|Default|SetRedClosed (Class|PrimitiveComponent|IsOverlappingComponent OverlappedComponent (Variables|Default|GetSphere%201))))

(event OnComponentBeginOverlap(SphereDoor5)
  (params (OverlappedComponent :type Primitive%20Component%20Object%20Reference) (OtherActor :type Actor%20Object%20Reference) (OtherComp :type Primitive%20Component%20Object%20Reference) (OtherBodyIndex :type Integer) (bFromSweep :type Boolean) (SweepResult :type Hit%20Result%20Structure%20%28by%20ref%29))
  ;[1 1 1] Blue Door Check
  (Variables|Default|SetBlueClosed (Class|PrimitiveComponent|IsOverlappingComponent OverlappedComponent (Variables|Default|GetSphere%202))))

(event OnComponentEndOverlap(SphereDoor5)
  (params (OverlappedComponent :type Primitive%20Component%20Object%20Reference) (OtherActor :type Actor%20Object%20Reference) (OtherComp :type Primitive%20Component%20Object%20Reference) (OtherBodyIndex :type Integer))
  ;[1 1 1] Blue Door Check
  (Variables|Default|SetBlueClosed (Class|PrimitiveComponent|IsOverlappingComponent OverlappedComponent (Variables|Default|GetSphere%202))))

(event OnComponentEndOverlap(SphereDoor4)
  (params (OverlappedComponent :type Primitive%20Component%20Object%20Reference) (OtherActor :type Actor%20Object%20Reference) (OtherComp :type Primitive%20Component%20Object%20Reference) (OtherBodyIndex :type Integer))
  ;[1 1 1] Red Door Check
  (Variables|Default|SetRedClosed (Class|PrimitiveComponent|IsOverlappingComponent OverlappedComponent (Variables|Default|GetSphere%201))))

(event Custom|Spawn%20Red
  (Game|SpawnActorfromClass "/Game/VRE/Blueprints/Postage/BP_PostageItem_Red.BP_PostageItem_Red_C" (Math|Transform|MakeTransform (Transformation|GetWorldLocation (Variables|Default|GetBillboard)) "0, 0, 0" "1.000000,1.000000,1.000000") "Undefined" "MultiplyWithRoot" 0 0))

(event Custom|Spawn%20Blue
  (Game|SpawnActorfromClass "/Game/VRE/Blueprints/Postage/BP_PostageItem_Blue.BP_PostageItem_Blue_C" (Math|Transform|MakeTransform (Transformation|GetWorldLocation (Variables|Default|GetBillboard1)) "0, 0, 0" "1.000000,1.000000,1.000000") "Undefined" "MultiplyWithRoot" 0 0))

(event Custom|Spawn%20Yellow
  (Game|SpawnActorfromClass "/Game/VRE/Blueprints/Postage/BP_PostageItem_Yellow.BP_PostageItem_Yellow_C" (Math|Transform|MakeTransform (Transformation|GetWorldLocation (Variables|Default|GetBillboard3)) "0, 0, 0" "1.000000,1.000000,1.000000") "Undefined" "MultiplyWithRoot" 0 0))

(event Custom|Spawn%20Green
  (Game|SpawnActorfromClass "/Game/VRE/Blueprints/Postage/BP_PostageItem_Green.BP_PostageItem_Green_C" (Math|Transform|MakeTransform (Transformation|GetWorldLocation (Variables|Default|GetBillboard2)) "0, 0, 0" "1.000000,1.000000,1.000000") "Undefined" "MultiplyWithRoot" 0 0))

(event Collision|EventActorBeginOverlap
  (params (OtherActor :type Actor%20Object%20Reference)))

(event EventBeginPlay)

(fn ConstructionScript)