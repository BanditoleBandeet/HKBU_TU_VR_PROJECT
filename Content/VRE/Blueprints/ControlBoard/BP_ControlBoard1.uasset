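; VR control board Blueprint with a marker plane and a VR render target manager, used to map world-space hits to render target pixels.
; CalcRelativePos projects the hit onto the plane in local space, offsets it by half the bounds and clamps it using the plane's X size.
; It then divides by a fixed 100 and scales by render target size.
; The events, construction script and board-data OnRep are empty.
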(event Collision|EventActorBeginOverlap
  (params (OtherActor :type Actor%20Object%20Reference)))

(event EventTick
  (params (DeltaSeconds :type Float%20%28single-precision%29)))

(fn ConstructionScript)

(fn CalcRelativePos
  (params (WorldSpaceHit :type Vector))
  (bind _markerplane (Variables|Default|GetMarkerPlane))
  (bind _vrrendertargetmanager (Variables|Default|GetVRRenderTargetManager))
  (bind _returnvalue (Transformation|GetWorldTransform _markerplane))
  (bind (_min _max) (Components|StaticMesh|GetLocalBounds _markerplane))
  (bind _rendertarget (Variables|/Script/VRExpansionPlugin.VRRenderTargetManager|GetRenderTarget _vrrendertargetmanager))
  (bind _returnvalue_2 (Math|Transform|InverseTransformLocation _returnvalue WorldSpaceHit))
  (bind _returnvalue_3 (- _max _min))
  (bind (_width _height) (Class|CanvasRenderTarget2D|GetSize _rendertarget))
  (bind _returnvalue_4 (/ _returnvalue_3 2.0))
  (bind _returnvalue_5 (Class|KismetMathLibrary|ProjectPointontoPlane _returnvalue_2 "0, 0, 0" "0, 0,1.000000"))
  (bind _returnvalue_6 (+ _returnvalue_5 _returnvalue_4))
  (bind (_x _y) (Math|Vector|BreakVector _returnvalue_6))
  (return (* (/ (Class|KismetMathLibrary|ClampAxes2D (Math|Vector2D|MakeVector2D _x _y) 0.0 (.X (Math|Vector|BreakVector _returnvalue_3))) 1e+02) (Math|Vector2D|MakeVector2D (Math|Conversions|ToFloat(Integer) _width) (Math|Conversions|ToFloat(Integer) _height)))) ; Hit Loc In UV
)

(fn OnRepReplicatedBoardData)