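; BP_PhysicalHandsSwap is a trigger actor that switches a VR character between physical grasping hands and regular grasping hands.
; It has three pairs of overlap components, one per mode, named SetPhysicalHands and SetGraspingHands.
; When a BP_VRCharacter begins overlapping one, it sets UsePhysicalGraspingHands to true or false to match that component.
; It only writes this flag on entry, with no end-overlap handling.
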(event OnComponentBeginOverlap(SetPhysicalHands01)
  (params (OverlappedComponent :type Primitive%20Component%20Object%20Reference) (OtherActor :type Actor%20Object%20Reference) (OtherComp :type Primitive%20Component%20Object%20Reference) (OtherBodyIndex :type Integer) (bFromSweep :type Boolean) (SweepResult :type Hit%20Result%20Structure%20%28by%20ref%29))
  (bind _asbp_vrcharacter (Utilities|Casting|CastToBP_VRCharacter OtherActor))
  (Variables|/Game/VRE/Core/Character/BP_VRCharacter.BP_VRCharacter_C|SetUsePhysicalGraspingHands _asbp_vrcharacter true))

(event OnComponentBeginOverlap(SetGraspingHands01)
  (params (OverlappedComponent :type Primitive%20Component%20Object%20Reference) (OtherActor :type Actor%20Object%20Reference) (OtherComp :type Primitive%20Component%20Object%20Reference) (OtherBodyIndex :type Integer) (bFromSweep :type Boolean) (SweepResult :type Hit%20Result%20Structure%20%28by%20ref%29))
  (bind _asbp_vrcharacter (Utilities|Casting|CastToBP_VRCharacter OtherActor))
  (Variables|/Game/VRE/Core/Character/BP_VRCharacter.BP_VRCharacter_C|SetUsePhysicalGraspingHands _asbp_vrcharacter false))

(event OnComponentBeginOverlap(SetGraspingHands02)
  (params (OverlappedComponent :type Primitive%20Component%20Object%20Reference) (OtherActor :type Actor%20Object%20Reference) (OtherComp :type Primitive%20Component%20Object%20Reference) (OtherBodyIndex :type Integer) (bFromSweep :type Boolean) (SweepResult :type Hit%20Result%20Structure%20%28by%20ref%29))
  (bind _asbp_vrcharacter (Utilities|Casting|CastToBP_VRCharacter OtherActor))
  (Variables|/Game/VRE/Core/Character/BP_VRCharacter.BP_VRCharacter_C|SetUsePhysicalGraspingHands _asbp_vrcharacter false))

(event OnComponentBeginOverlap(SetPhysicalHands02)
  (params (OverlappedComponent :type Primitive%20Component%20Object%20Reference) (OtherActor :type Actor%20Object%20Reference) (OtherComp :type Primitive%20Component%20Object%20Reference) (OtherBodyIndex :type Integer) (bFromSweep :type Boolean) (SweepResult :type Hit%20Result%20Structure%20%28by%20ref%29))
  (bind _asbp_vrcharacter (Utilities|Casting|CastToBP_VRCharacter OtherActor))
  (Variables|/Game/VRE/Core/Character/BP_VRCharacter.BP_VRCharacter_C|SetUsePhysicalGraspingHands _asbp_vrcharacter true))

(event OnComponentBeginOverlap(SetPhysicalHands03)
  (params (OverlappedComponent :type Primitive%20Component%20Object%20Reference) (OtherActor :type Actor%20Object%20Reference) (OtherComp :type Primitive%20Component%20Object%20Reference) (OtherBodyIndex :type Integer) (bFromSweep :type Boolean) (SweepResult :type Hit%20Result%20Structure%20%28by%20ref%29))
  (bind _asbp_vrcharacter (Utilities|Casting|CastToBP_VRCharacter OtherActor))
  (Variables|/Game/VRE/Core/Character/BP_VRCharacter.BP_VRCharacter_C|SetUsePhysicalGraspingHands _asbp_vrcharacter true))

(event OnComponentBeginOverlap(SetGraspingHands03)
  (params (OverlappedComponent :type Primitive%20Component%20Object%20Reference) (OtherActor :type Actor%20Object%20Reference) (OtherComp :type Primitive%20Component%20Object%20Reference) (OtherBodyIndex :type Integer) (bFromSweep :type Boolean) (SweepResult :type Hit%20Result%20Structure%20%28by%20ref%29))
  (bind _asbp_vrcharacter (Utilities|Casting|CastToBP_VRCharacter OtherActor))
  (Variables|/Game/VRE/Core/Character/BP_VRCharacter.BP_VRCharacter_C|SetUsePhysicalGraspingHands _asbp_vrcharacter false))

(event EventBeginPlay)

(event Collision|EventActorBeginOverlap
  (params (OtherActor :type Actor%20Object%20Reference)))

(event EventTick
  (params (DeltaSeconds :type Float%20%28single-precision%29)))

(fn ConstructionScript)