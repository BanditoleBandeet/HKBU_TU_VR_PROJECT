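; Golden bun tower collectable that plays a celebratory pickup sequence once when a VR character overlaps its capsule.
; Three timelines, rate-scaled by length variables, lift the mesh to a target height, speed up its rotating movement and shrink it toward zero.
; A 7.5-second delay, started from the scale-down update, leads to explosion and victory sounds, sparks, actor destruction and removal of the bun collection and indicator 3D widgets.
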(event OnComponentBeginOverlap(Capsule)
  (params (OverlappedComponent :type Primitive%20Component%20Object%20Reference) (OtherActor :type Actor%20Object%20Reference) (OtherComp :type Primitive%20Component%20Object%20Reference) (OtherBodyIndex :type Integer) (bFromSweep :type Boolean) (SweepResult :type Hit%20Result%20Structure%20%28by%20ref%29))
  (bind _self self)
  (bind _self_2 self)
  (bind _sm_goldbuntowercollectable (Variables|Default|GetSM_GoldBunTowerCollectable _self))
  (bind _sm_goldbuntowercollectable_2 (Variables|Default|GetSM_GoldBunTowerCollectable _self_2))
  (bind _returnvalue (Transformation|GetWorldLocation _sm_goldbuntowercollectable))
  (bind _returnvalue_2 (Transformation|GetWorldLocation _sm_goldbuntowercollectable_2))
  (Utilities|Casting|CastToBP_VRCharacter OtherActor)
  (Utilities|FlowControl|DoOnce false
    (:Completed
      (Audio|PlaySoundatLocation "/Game/VRE/SFX/Whoosh/Big/whoosh.whoosh" (Transformation|GetWorldLocation _sm_goldbuntowercollectable_2) "0, 0, 0" 1.0 1.0 0.0 0 0 0 0)
      (Utilities|FlowControl|Sequence
        (:then_0
          ;[1 1 1] Bun Fly Into Air
          (Components|Timeline|SetPlayRate (Variables|Default|GetGoldBunFlyIntoAir) (/ 1.0 (Variables|Timeline|GetTimelineBunFlyIntoAirLength)))
          (bind _lerp0_1 (Timeline|GoldBunFlyIntoAir PlayFromStart)
            (:Update
              (if (not (Utilities|Operators|EqualEqual (Math|Vector|Lerp(Vector) (Math|Vector|MakeVector (.x _returnvalue_2) (.y _returnvalue_2) (.z _returnvalue_2)) (Math|Vector|MakeVector (.x _returnvalue_2) (.y _returnvalue_2) (Variables|Default|GetTarget%20Z%20Height)) _lerp0_1) (Math|Vector|MakeVector (.x _returnvalue_2) (.y _returnvalue_2) (Variables|Default|GetTarget%20Z%20Height)) 0.0))
                (Transformation|SetWorldLocation (Variables|Default|GetSM_GoldBunTowerCollectable) (Math|Vector|Lerp(Vector) (Math|Vector|MakeVector (.x _returnvalue_2) (.y _returnvalue_2) (.z _returnvalue_2)) (Math|Vector|MakeVector (.x _returnvalue_2) (.y _returnvalue_2) (Variables|Default|GetTarget%20Z%20Height)) _lerp0_1) false false)))))
        (:then_1
          ;[1 1 1] Bun Rotation Speed Up
          (Components|Timeline|SetPlayRate (Variables|Default|GetGoldBunRotationSpeedUp) (/ 1.0 (Variables|Timeline|GetTimelineBunRotationSpeedUpLength)))
          (bind _lerp_0_1 (Timeline|GoldBunRotationSpeedUp PlayFromStart)
            (:Update
              (Variables|/Script/Engine.RotatingMovementComponent|SetRotationRate (Variables|Default|GetRotatingMovement) (Math|Rotator|Lerp(Rotator) (Variables|/Script/Engine.RotatingMovementComponent|GetRotationRate (Variables|Default|GetRotatingMovement)) (Variables|Default|GetCollectionRotationTarget) _lerp_0_1)))))
        (:then_2
          ;[1 1 1] Bun scale down
          (Components|Timeline|SetPlayRate (Variables|Default|GetGoldBunScaleDown) (/ 1.0 (Variables|Timeline|GetTimelineBunScaleDownLength)))
          (bind _lerp_0_1_2 (Timeline|GoldBunScaleDown PlayFromStart)
            (:Update
              (Transformation|SetRelativeScale3D (Variables|Default|GetSM_GoldBunTowerCollectable) (Math|Vector|Lerp(Vector) (Transformation|GetWorldScale (Variables|Default|GetSM_GoldBunTowerCollectable)) "0, 0, 0" _lerp_0_1_2))
              (Utilities|FlowControl|Delay 7.5)
              (Audio|PlaySoundatLocation "/Game/StarterContent/Audio/Explosion02.Explosion02" _returnvalue "0, 0, 0" 1.0 1.0 0.0 0 0 0 0)
              (Effects|SpawnEmitteratLocation "/Game/Realistic_Starter_VFX_Pack_Vol2/Particles/Sparks/P_Sparks_G.P_Sparks_G" _returnvalue "0, 0, 0" "2.000000,2.000000,2.000000")
              (Audio|PlaySound2D "/Game/VRE/SFX/Victory/victory.victory" 1.0 1.0 0.0 0 0)
              (Actor|DestroyActor)
              (bind _outactors (Actor|GetAllActorsOfClass "/Game/VRE/UI/BunTowerProgressScreen/BunsCollect3DWidget.BunsCollect3DWidget_C"))
              (for _array_element _outactors
                (Actor|DestroyActor _array_element)
                (bind _outactors_2 (Actor|GetAllActorsOfClass "/Game/VRE/Blueprints/BunTower/BP_3DWidgetBunIndicator.BP_3DWidgetBunIndicator_C"))
                (for _array_element_2 _outactors_2
                  (Actor|DestroyActor _array_element_2))))))))))

(fn ConstructionScript)