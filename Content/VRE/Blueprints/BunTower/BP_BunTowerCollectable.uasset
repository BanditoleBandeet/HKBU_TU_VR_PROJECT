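; VR collectable bun for the BunTower area that a BP_VRCharacter picks up by overlapping its box, adding one to that character's collected count.
; Pickup fires once, playing a whoosh and a spin timeline that lerps rotation rate.
; Each spin update restarts a shrink timeline that scales bun and sparkles toward zero.
; When shrinking finishes, it plays a munch sound, activates crumb Niagara VFX and immediately destroys itself.
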(event OnComponentBeginOverlap(Box)
  (params (OverlappedComponent :type Primitive%20Component%20Object%20Reference) (OtherActor :type Actor%20Object%20Reference) (OtherComp :type Primitive%20Component%20Object%20Reference) (OtherBodyIndex :type Integer) (bFromSweep :type Boolean) (SweepResult :type Hit%20Result%20Structure%20%28by%20ref%29))
  (bind _asbp_vrcharacter (Utilities|Casting|CastToBP_VRCharacter OtherActor))
  (Utilities|FlowControl|DoOnce false
    (:Completed
      (Variables|/Game/VRE/Core/Character/BP_VRCharacter.BP_VRCharacter_C|SetCurrentBunTowerCollectablesCollected _asbp_vrcharacter (+ (Variables|/Game/VRE/Core/Character/BP_VRCharacter.BP_VRCharacter_C|GetCurrentBunTowerCollectablesCollected _asbp_vrcharacter) 1))
      (Audio|SpawnSoundatLocation "/Game/VRE/SFX/Whoosh/Small/smallwhoosh.smallwhoosh" (Transformation|GetWorldLocation (Variables|Default|GetSM_BunTowerCollectable)) "0, 0, 0" 1.0 1.0 0.0 0 0)
      (bind _bunspincollection (Timeline|BunSpinCollection PlayFromStart)
        (:Update
          (Variables|/Script/Engine.RotatingMovementComponent|SetRotationRate (Variables|Default|GetRotatingMovement) (Math|Rotator|Lerp(Rotator) (Variables|/Script/Engine.RotatingMovementComponent|GetRotationRate (Variables|Default|GetRotatingMovement)) (Variables|Default|GetCollectionRotationTarget) _bunspincollection))
          (bind _bungrowsmaller (Timeline|BunGrowSmaller PlayFromStart)
            (:Update
              (Transformation|SetRelativeScale3D (Variables|Default|GetSM_BunTowerCollectable) (Math|Vector|Lerp(Vector) (Transformation|GetWorldScale (Variables|Default|GetSM_BunTowerCollectable)) "0, 0, 0" _bungrowsmaller))
              (Transformation|SetWorldScale3D (Variables|Default|GetSparkleParticleSystem) (Math|Vector|Lerp(Vector) (Variables|Default|GetDefaultSparklesVector) "0, 0, 0" _bungrowsmaller)))
            (:Finished
              (CallFunction|BunCollected))))))))

(event Custom|BunCollected
  (Audio|PlaySoundatLocation "/Game/VRE/SFX/Eating/EatMunch.EatMunch" (Transformation|GetWorldLocation (Variables|Default|GetSM_BunTowerCollectable self)) "0, 0, 0" 1.0 1.0 0.0 0 0 0 0)
  (Components|Activation|Activate (Variables|Default|GetNiagaraCrumbVFX) false)
  (Actor|DestroyActor))

(event EventBeginPlay)

(fn ConstructionScript)