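; BP_BunSpawner places BP_BunTowerCollectable actors at a random selection of predefined spots for the bun tower.
; On BeginPlay it appends BunTransforms to a working list, then spawns TotalBunToSpawn collectables at randomly picked entries, converting each location from the spawner's local space to world space.
; Each picked entry is removed from the working list, so picks do not reuse the same entry.
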(event EventBeginPlay
  (bind _temp_bun_transforms (Variables|Default|GetTEMP_Bun_Transforms))
  (bind _temp_bun_transforms_2 (Variables|Default|GetTEMP_Bun_Transforms))
  (Utilities|Array|AppendArray _temp_bun_transforms_2 (Variables|Default|GetBun_Transforms))
  (for _index (range 0 (- (Variables|Default|GetTotalBunToSpawn) 1))
    (Variables|Default|SetChosenbunTransform (Math|Random|RandomIntegerinRange 0 (- (Utilities|Array|Length _temp_bun_transforms_2) 1)))
    (Game|SpawnActorfromClass "/Game/VRE/Blueprints/BunTower/BP_BunTowerCollectable.BP_BunTowerCollectable_C" (Math|Transform|MakeTransform (Math|Transform|TransformLocation (Transformation|GetActorTransform) (.location (Utilities|Array|Get(acopy) (Variables|Default|GetTEMP_Bun_Transforms) (Variables|Default|GetChosenbunTransform)))) "0, 0, 0" "1.000000,1.000000,1.000000") "Undefined" "MultiplyWithRoot" 0 0)
    (Utilities|Array|RemoveItem _temp_bun_transforms (Utilities|Array|Get(acopy) _temp_bun_transforms (Variables|Default|GetChosenbunTransform)))))

(fn ConstructionScript)