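; BP_Lever is a VR lever actor that acts as a zoom control for the binoculars stand.
; Every tick it finds all BP_BinocsStand actors and copies the VRLever's current angle directly into the first one's scene capture FOV, with no remapping or clamping.
; It also prints the resulting FOV each frame, and the lookup is neither cached nor checked for an empty result.
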(event EventBeginPlay
  (|CallParentFunction) ; This node is disabled and will not be called.\nDrag off pins to build functionality.
)

(event Collision|EventActorBeginOverlap
  (params (OtherActor :type Actor%20Object%20Reference))
  (|CallParentFunction OtherActor) ; This node is disabled and will not be called.\nDrag off pins to build functionality.
)

(event EventTick
  (params (DeltaSeconds :type Float%20%28single-precision%29))
  (|CallParentFunction DeltaSeconds)
  (bind _outactors (Actor|GetAllActorsOfClass "/Game/VRE/Blueprints/BinocsStand/BP_BinocsStand.BP_BinocsStand_C"))
  (bind _output_get (Variables|/Script/Engine.SceneCaptureComponent2D|SetFOVAngle (Variables|/Game/VRE/Blueprints/BinocsStand/BP_BinocsStand.BP_BinocsStand_C|GetSceneCaptureComponent2D (Utilities|Array|Get(acopy) _outactors)) (Variables|/Script/VRExpansionPlugin.VRLeverComponent|GetCurrentLeverAngle (Variables|Default|GetVRLever))))
  (Development|PrintString (Utilities|String|ToString(Float) _output_get)))

(fn ConstructionScript
  (|CallParentFunction))