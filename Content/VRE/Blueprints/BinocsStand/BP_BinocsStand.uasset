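; BP_BinocsStand is a VR binoculars stand actor with a lever-driven Plane and a SceneCaptureComponent2D.
; BeginPlay narrows the capture's field of view for a zoomed-in view.
; Every Tick sets the Plane's world roll from the VRLever's current angle plus an offset, with pitch and yaw fixed in world space.
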(event EventBeginPlay
  (Variables|/Script/Engine.SceneCaptureComponent2D|SetFOVAngle (Variables|Default|GetSceneCaptureComponent2D) 1e+01))

(event Collision|EventActorBeginOverlap
  (params (OtherActor :type Actor%20Object%20Reference)))

(event EventTick
  (params (DeltaSeconds :type Float%20%28single-precision%29))
  (Transformation|SetWorldRotation (Variables|Default|GetPlane) (Math|Rotator|MakeRotator (+ (Variables|/Script/VRExpansionPlugin.VRLeverComponent|GetCurrentLeverAngle (Variables|Default|GetVRLever)) 9e+01) 0.0 9e+01) false false))

(fn ConstructionScript)