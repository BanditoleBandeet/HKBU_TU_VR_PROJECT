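; VR button actor that steps the zoom of the binoculars stand.
; Each state change of its ButtonComp finds the first BP_BinocsStand in the level and lowers that stand's SceneCaptureComponent2D field of view by a fixed step.
; Once the view narrows to the lower limit it wraps back to wide, so repeated use cycles through zoom levels.
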(event OnButtonStateChanged(ButtonComp)
  (params (ButtonState :type Boolean) (InteractingActor :type Actor%20Object%20Reference) (InteractingComponent :type Primitive%20Component%20Object%20Reference))
  (bind _outactors (Actor|GetAllActorsOfClass "/Game/VRE/Blueprints/BinocsStand/BP_BinocsStand.BP_BinocsStand_C"))
  (bind _output_get (Variables|/Script/Engine.SceneCaptureComponent2D|SetFOVAngle (Variables|/Game/VRE/Blueprints/BinocsStand/BP_BinocsStand.BP_BinocsStand_C|GetSceneCaptureComponent2D (Utilities|Array|Get(acopy) _outactors)) (- (Variables|/Script/Engine.SceneCaptureComponent2D|GetFOVAngle (Variables|/Game/VRE/Blueprints/BinocsStand/BP_BinocsStand.BP_BinocsStand_C|GetSceneCaptureComponent2D (Utilities|Array|Get(acopy) _outactors))) 2e+01)))
  (if (<= _output_get 1e+01)
    (Variables|/Script/Engine.SceneCaptureComponent2D|SetFOVAngle (Variables|/Game/VRE/Blueprints/BinocsStand/BP_BinocsStand.BP_BinocsStand_C|GetSceneCaptureComponent2D (Utilities|Array|Get(acopy) _outactors)) 9e+01)))

(event EventBeginPlay
  (|CallParentFunction) ; This node is disabled and will not be called.\nDrag off pins to build functionality.
)

(event Collision|EventActorBeginOverlap
  (params (OtherActor :type Actor%20Object%20Reference)))

(event EventTick
  (params (DeltaSeconds :type Float%20%28single-precision%29))
  (|CallParentFunction DeltaSeconds) ; This node is disabled and will not be called.\nDrag off pins to build functionality.
)

(fn ConstructionScript
  (|CallParentFunction))