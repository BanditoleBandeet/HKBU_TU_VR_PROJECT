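; BP_Firework is a VR firework that is armed when used and launches when the grip is released.
; On launch, a timeline with its play rate scaled by TimelineLength moves the actor along its arrow's forward vector by a fixed step each update.
; After a delay, a DoOnce plays audio and activates the VFX once, then the actor destroys itself shortly afterwards.
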(event Custom|FireworkEvent
  (Components|Timeline|SetPlayRate (Variables|Default|GetTimeline) (/ 1.0 (Variables|Default|Gettimeline%20length)))
  (Timeline|Timeline PlayFromStart
    (:Update
      (Transformation|SetActorLocation (+ (Transformation|GetActorLocation) (* (Math|Vector|GetForwardVector (Variables|Default|GetArrow)) 3e+01)) false false)
      (Utilities|FlowControl|Delay 2.0)
      (Utilities|FlowControl|DoOnce false
        (:Completed
          (Audio|Components|Audio|Play (Variables|Default|GetAudio) 0.0)
          (Components|Activation|Activate (Variables|Default|GetVFX) false)
          (Utilities|FlowControl|Delay 0.2)
          (Actor|DestroyActor))))))

(event EventOnUsed
  (Variables|Default|SetHasClicked true))

(event EventOnGripRelease
  (params (ReleasingController :type Grip%20Motion%20Controller%20Component%20Object%20Reference) (GripInformation :type BP%20Actor%20Grip%20Information%20Structure%20%28by%20ref%29) (bWasSocketed :type Boolean))
  (if (Variables|Default|GetHasClicked)
    (CallFunction|FireworkEvent)))

(fn ConstructionScript)