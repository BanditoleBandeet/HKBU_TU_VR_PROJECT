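; BP_SnowmanArms1 is an interactable snowman arms piece that can be placed on a snowman's middle section.
; Capsule overlaps with BP_SnowmanMiddle1 toggle an Interacting flag.
; When used while that flag is set, it plays a snow crumple sound and spawns a copy of itself at its mesh's world location and rotation.
; The copy's mesh collision is set to query only, and the original actor remains.
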(event OnComponentBeginOverlap(Capsule)
  (params (OverlappedComponent :type Primitive%20Component%20Object%20Reference) (OtherActor :type Actor%20Object%20Reference) (OtherComp :type Primitive%20Component%20Object%20Reference) (OtherBodyIndex :type Integer) (bFromSweep :type Boolean) (SweepResult :type Hit%20Result%20Structure%20%28by%20ref%29))
  (Utilities|Casting|CastToBP_SnowmanMiddle1 OtherActor)
  (Variables|Default|SetInteracting true))

(event OnComponentEndOverlap(Capsule)
  (params (OverlappedComponent :type Primitive%20Component%20Object%20Reference) (OtherActor :type Actor%20Object%20Reference) (OtherComp :type Primitive%20Component%20Object%20Reference) (OtherBodyIndex :type Integer))
  (Utilities|Casting|CastToBP_SnowmanMiddle1 OtherActor)
  (Variables|Default|SetInteracting false))

(event Custom|Place%20Object
  (bind _staticmeshcomponent (Variables|Default|GetStaticMeshComponent))
  (bind _returnvalue (Game|SpawnActorfromClass "BP_SnowmanArms1_C" (Math|Transform|MakeTransform (Transformation|GetWorldLocation _staticmeshcomponent) (Transformation|GetWorldRotation _staticmeshcomponent) "1.000000,1.000000,1.000000") "Undefined" "MultiplyWithRoot" 0 0))
  (Collision|SetCollisionEnabled (Variables|/Script/Engine.StaticMeshActor|GetStaticMeshComponent _returnvalue) "QueryOnly"))

(event EventOnUsed
  (if (Variables|Default|GetInteracting)
    (Audio|PlaySound2D "/Game/VRE/Blueprints/Snowman/Snowman/SnowCrumple.SnowCrumple" 1.0 1.0 0.0 0 0)
    (CallFunction|PlaceObject)))

(fn ConstructionScript)