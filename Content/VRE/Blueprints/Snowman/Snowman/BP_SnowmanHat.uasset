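; BP_SnowmanHat is a grippable hat that can be placed on a snowman.
; A box overlap with BP_SnowmanTop sets an Interacting flag.
; Using the hat while flagged plays a snow crumple sound, then replaces it with a new copy at the mesh's transform, set to query-and-probe collision.
; Releasing the grip destroys the hat after a short delay and spawns a fresh one at HatSpawn.
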(event OnComponentBeginOverlap(Box)
  (params (OverlappedComponent :type Primitive%20Component%20Object%20Reference) (OtherActor :type Actor%20Object%20Reference) (OtherComp :type Primitive%20Component%20Object%20Reference) (OtherBodyIndex :type Integer) (bFromSweep :type Boolean) (SweepResult :type Hit%20Result%20Structure%20%28by%20ref%29))
  (Utilities|Casting|CastToBP_SnowmanTop OtherActor)
  (Variables|Default|SetInteracting true))

(event OnComponentEndOverlap(Box)
  (params (OverlappedComponent :type Primitive%20Component%20Object%20Reference) (OtherActor :type Actor%20Object%20Reference) (OtherComp :type Primitive%20Component%20Object%20Reference) (OtherBodyIndex :type Integer))
  (Utilities|Casting|CastToBP_SnowmanTop OtherActor)
  (Variables|Default|SetInteracting false))

(event Custom|PlaceObject
  (bind _staticmeshcomponent (Variables|Default|GetStaticMeshComponent))
  (bind _returnvalue (Game|SpawnActorfromClass "BP_SnowmanHat_C" (Math|Transform|MakeTransform (Transformation|GetWorldLocation _staticmeshcomponent) (Transformation|GetWorldRotation _staticmeshcomponent) "1.000000,1.000000,1.000000") "Undefined" "MultiplyWithRoot" 0 0))
  (Collision|SetCollisionEnabled (Variables|/Script/Engine.StaticMeshActor|GetStaticMeshComponent _returnvalue) "QueryAndProbe"))

(event EventBeginPlay)

(event Collision|EventActorBeginOverlap
  (params (OtherActor :type Actor%20Object%20Reference)))

(event EventTick
  (params (DeltaSeconds :type Float%20%28single-precision%29)))

(event EventOnUsed
  (if (Variables|Default|GetInteracting)
    (Audio|PlaySound2D "/Game/VRE/Blueprints/Snowman/Snowman/SnowCrumple.SnowCrumple" 1.0 1.0 0.0 0 0)
    (CallFunction|PlaceObject)
    (Actor|DestroyActor)))

(event EventOnGripRelease
  (params (ReleasingController :type Grip%20Motion%20Controller%20Component%20Object%20Reference) (GripInformation :type BP%20Actor%20Grip%20Information%20Structure%20%28by%20ref%29) (bWasSocketed :type Boolean))
  (Utilities|FlowControl|Delay 1.0)
  (Actor|DestroyActor)
  (Game|SpawnActorfromClass "BP_SnowmanHat_C" (Math|Transform|MakeTransform (Variables|Default|GetHatSpawn) "0, 0, 0" "1.000000,1.000000,1.000000") "Undefined" "MultiplyWithRoot" 0 0))

(fn ConstructionScript)