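; A button actor that starts the snowman-building sequence by spawning the snowman's parts.
; When its button component changes state, a DoOnce gate lets it spawn the middle, top, hat, carrot, stones and arms at preset spawn transforms.
; On each press it also binds to the first BP_ButtonSnowmanRestart found in the level, whose restart event resets the gate so the parts can spawn again.
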(event OnButtonStateChanged(ButtonComp)
  (params (ButtonState :type Boolean) (InteractingActor :type Actor%20Object%20Reference) (InteractingComponent :type Primitive%20Component%20Object%20Reference))
  (bind _outactors (Actor|GetAllActorsOfClass "/Game/VRE/Blueprints/Snowman/Snowman/BP_ButtonSnowmanRestart.BP_ButtonSnowmanRestart_C"))
  (EventDispatchers|BindEventtoSnowmanRestart (Utilities|Array|Get(acopy) _outactors) (delegate Custom|If%20restarted%20allow%202nd%20spawning))
  (Utilities|FlowControl|DoOnce false
    (:Completed
      (Utilities|FlowControl|Sequence
        (:then_0
          (Game|SpawnActorfromClass "/Game/VRE/Blueprints/Snowman/Snowman/BP_SnowmanMiddle1.BP_SnowmanMiddle1_C" (Math|Transform|MakeTransform (Variables|Default|GetMiddleSpawn) "0, 0, 0" "1.000000,1.000000,1.000000") "Undefined" "MultiplyWithRoot" 0 0))
        (:then_1
          (Game|SpawnActorfromClass "/Game/VRE/Blueprints/Snowman/Snowman/BP_SnowmanTop.BP_SnowmanTop_C" (Math|Transform|MakeTransform (Variables|Default|GetTopSpawn) "0, 0, 0" "1.000000,1.000000,1.000000") "Undefined" "MultiplyWithRoot" 0 0))
        (:then_2
          (Game|SpawnActorfromClass "/Game/VRE/Blueprints/Snowman/Snowman/BP_SnowmanHat.BP_SnowmanHat_C" (Math|Transform|MakeTransform (Variables|Default|GetHatSpawn) "0, 0, 0" "1.000000,1.000000,1.000000") "Undefined" "MultiplyWithRoot" 0 0))
        (:then_3
          (Game|SpawnActorfromClass "/Game/VRE/Blueprints/Snowman/Snowman/BP_SnowmanCarrot.BP_SnowmanCarrot_C" (Math|Transform|MakeTransform (Variables|Default|GetCarrotSpawn) "0, 0, 0" "1.000000,1.000000,1.000000") "Undefined" "MultiplyWithRoot" 0 0))
        (:then_4
          (Game|SpawnActorfromClass "/Game/VRE/Blueprints/Snowman/Snowman/BP_SnowmanStones.BP_SnowmanStones_C" (Math|Transform|MakeTransform (Variables|Default|GetStoneSpawn) "0, 0, 0" "1.000000,1.000000,1.000000") "Undefined" "MultiplyWithRoot" 0 0))
        (:then_5
          (Game|SpawnActorfromClass "/Game/VRE/Blueprints/Snowman/Snowman/BP_SnowmanArms1.BP_SnowmanArms1_C" (Math|Transform|MakeTransform (Variables|Default|GetArmSpawn) "0, 0, 0" "1.000000,1.000000,1.000000") "Undefined" "MultiplyWithRoot" 0 0))))))

(event Custom|If%20restarted%20allow%202nd%20spawning
  (Utilities|FlowControl|DoOnce false) ; enters at Reset
)

(event EventBeginPlay
  (|CallParentFunction) ; This node is disabled and will not be called.\nDrag off pins to build functionality.
)

(event Collision|EventActorBeginOverlap
  (params (OtherActor :type Actor%20Object%20Reference)))

(event EventTick
  (params (DeltaSeconds :type Float%20%28single-precision%29))
  (|CallParentFunction DeltaSeconds) ; This node is disabled and will not be called.\nDrag off pins to build functionality.
)

(fn ConstructionScript
  (|CallParentFunction))