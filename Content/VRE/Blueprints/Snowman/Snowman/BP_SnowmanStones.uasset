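; BP_SnowmanStones is a usable stone prop for decorating a snowman's top piece.
; A sphere overlap with BP_SnowmanTop toggles an Interacting flag that gates the OnUsed event.
; Using it while overlapping spawns another BP_SnowmanStones at the mesh's world position and rotation, with query-only collision.
; The original actor remains, as the DestroyActor call is not connected.
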(event OnComponentBeginOverlap(Sphere)
  (params (OverlappedComponent :type Primitive%20Component%20Object%20Reference) (OtherActor :type Actor%20Object%20Reference) (OtherComp :type Primitive%20Component%20Object%20Reference) (OtherBodyIndex :type Integer) (bFromSweep :type Boolean) (SweepResult :type Hit%20Result%20Structure%20%28by%20ref%29))
  (Utilities|Casting|CastToBP_SnowmanTop OtherActor)
  (Variables|Default|SetInteracting true))

(event OnComponentEndOverlap(Sphere)
  (params (OverlappedComponent :type Primitive%20Component%20Object%20Reference) (OtherActor :type Actor%20Object%20Reference) (OtherComp :type Primitive%20Component%20Object%20Reference) (OtherBodyIndex :type Integer))
  (Utilities|Casting|CastToBP_SnowmanTop OtherActor)
  (Variables|Default|SetInteracting false))

(event Custom|PlaceObject
  (bind _staticmeshcomponent (Variables|Default|GetStaticMeshComponent))
  (bind _returnvalue (Game|SpawnActorfromClass "BP_SnowmanStones_C" (Math|Transform|MakeTransform (Transformation|GetWorldLocation _staticmeshcomponent) (Transformation|GetWorldRotation _staticmeshcomponent) "1.000000,1.000000,1.000000") "Undefined" "MultiplyWithRoot" 0 0))
  (Collision|SetCollisionEnabled (Variables|/Script/Engine.StaticMeshActor|GetStaticMeshComponent _returnvalue) "QueryOnly"))

(event EventOnUsed
  (if (Variables|Default|GetInteracting)
    (CallFunction|PlaceObject)))

(fn ConstructionScript)