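; VR button actor that resets the snowman-building activity by clearing the placed snowman parts.
; Any state change on its button component runs a sequence that finds and destroys all middle, top, hat, stones, arms and carrot actors by class.
; The SnowmanRestart dispatcher fires inside each loop, so listeners are notified once per destroyed actor rather than once per reset.
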(event OnButtonStateChanged(ButtonComp)
  (params (ButtonState :type Boolean) (InteractingActor :type Actor%20Object%20Reference) (InteractingComponent :type Primitive%20Component%20Object%20Reference))
  (Utilities|FlowControl|Sequence
    (:then_0
      (bind _outactors (Actor|GetAllActorsOfClass "/Game/VRE/Blueprints/Snowman/Snowman/BP_SnowmanMiddle1.BP_SnowmanMiddle1_C"))
      (for _array_element _outactors
        (Actor|DestroyActor _array_element)
        (Default|CallSnowmanRestart)))
    (:then_1
      (bind _outactors_2 (Actor|GetAllActorsOfClass "/Game/VRE/Blueprints/Snowman/Snowman/BP_SnowmanTop.BP_SnowmanTop_C"))
      (for _array_element_2 _outactors_2
        (Actor|DestroyActor _array_element_2)
        (Default|CallSnowmanRestart)))
    (:then_2
      (bind _outactors_3 (Actor|GetAllActorsOfClass "/Game/VRE/Blueprints/Snowman/Snowman/BP_SnowmanHat.BP_SnowmanHat_C"))
      (for _array_element_3 _outactors_3
        (Actor|DestroyActor _array_element_3)
        (Default|CallSnowmanRestart)))
    (:then_3
      (bind _outactors_4 (Actor|GetAllActorsOfClass "/Game/VRE/Blueprints/Snowman/Snowman/BP_SnowmanStones.BP_SnowmanStones_C"))
      (for _array_element_4 _outactors_4
        (Actor|DestroyActor _array_element_4)
        (Default|CallSnowmanRestart)))
    (:then_4
      (bind _outactors_5 (Actor|GetAllActorsOfClass "/Game/VRE/Blueprints/Snowman/Snowman/BP_SnowmanArms1.BP_SnowmanArms1_C"))
      (for _array_element_5 _outactors_5
        (Actor|DestroyActor _array_element_5)
        (Default|CallSnowmanRestart)))
    (:then_5
      (bind _outactors_6 (Actor|GetAllActorsOfClass "/Game/VRE/Blueprints/Snowman/Snowman/BP_SnowmanCarrot.BP_SnowmanCarrot_C"))
      (for _array_element_6 _outactors_6
        (Actor|DestroyActor _array_element_6)
        (Default|CallSnowmanRestart)))))

(event EventBeginPlay
  (|CallParentFunction) ; This node is disabled and will not be called.\nDrag off pins to build functionality.
)

(event Collision|EventActorBeginOverlap
  (params (OtherActor :type Actor%20Object%20Reference)))

(event EventTick
  (params (DeltaSeconds :type Float%20%28single-precision%29))
  (|CallParentFunction DeltaSeconds) ; This node is disabled and will not be called.\nDrag off pins to build functionality.
)

(fn ConstructionScript
  (|CallParentFunction))