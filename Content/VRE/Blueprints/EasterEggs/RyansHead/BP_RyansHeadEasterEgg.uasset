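; BP_RyansHeadEasterEgg is an Easter egg actor that raises the SMRyanKraken mesh into view and later lowers it again.
; ReleaseTheRyan fires once through a DoOnce and plays the MoveUpwards timeline, lerping the mesh between two hardcoded world positions along Z.
; After a six-second delay it calls Submerge, which reverses the same timeline.
; The timeline play-rate setup is unconnected and never runs.
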(event Custom|ReleaseTheRyan
  (Utilities|FlowControl|DoOnce false
    (:Completed
      (Utilities|FlowControl|Sequence
        (:then_0
          (bind _lerp_0_1 (Timeline|MoveUpwards PlayFromStart)
            (:Update
              (Transformation|SetWorldLocation (Variables|Default|GetSM_RyanKraken) (Math|Vector|Lerp(Vector) (Math|Vector|MakeVector -28964.571765 -57.600343 81.489581) (Math|Vector|MakeVector -28964.571765 -57.600343 613.767005) _lerp_0_1) false false))))
        (:then_1
          (Utilities|FlowControl|Delay 6.0)
          (CallFunction|Submerge))))))

(event Custom|Submerge
  (bind _lerp_0_1 (Timeline|MoveUpwards Reverse)
    (:Update
      (Transformation|SetWorldLocation (Variables|Default|GetSM_RyanKraken) (Math|Vector|Lerp(Vector) (Math|Vector|MakeVector -28964.571765 -57.600343 81.489581) (Math|Vector|MakeVector -28964.571765 -57.600343 613.767005) _lerp_0_1) false false))))

(fn ConstructionScript)