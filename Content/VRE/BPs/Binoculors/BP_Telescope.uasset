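; BP_Telescope is a VR telescope actor whose zoom changes each time it is used.
; OnUsed plays a click sound and narrows the SceneCaptureComponent2D field of view by a fixed step, magnifying the captured view.
; Near the narrow limit it subtracts a smaller step and resets to the wide angle in the same use, so repeated uses cycle through zoom levels.
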(event EventBeginPlay)

(event Collision|EventActorBeginOverlap
  (params (OtherActor :type Actor%20Object%20Reference)))

(event EventTick
  (params (DeltaSeconds :type Float%20%28single-precision%29)))

(event EventOnUsed
  (bind _scenecapturecomponent2d (Variables|Default|GetSceneCaptureComponent2D))
  (Audio|PlaySound2D "/Game/VRE/SFX/Click.Click" 1.0 1.0 0.0 0 0)
  (Variables|/Script/Engine.SceneCaptureComponent2D|SetFOVAngle _scenecapturecomponent2d (- (Variables|/Script/Engine.SceneCaptureComponent2D|GetFOVAngle _scenecapturecomponent2d) 2e+01))
  (if (<= (Variables|/Script/Engine.SceneCaptureComponent2D|GetFOVAngle _scenecapturecomponent2d) 1e+01)
    (Variables|/Script/Engine.SceneCaptureComponent2D|SetFOVAngle _scenecapturecomponent2d (- (Variables|/Script/Engine.SceneCaptureComponent2D|GetFOVAngle _scenecapturecomponent2d) 5.0))
    (if (<= (Variables|/Script/Engine.SceneCaptureComponent2D|GetFOVAngle _scenecapturecomponent2d) 5.0)
      (Variables|/Script/Engine.SceneCaptureComponent2D|SetFOVAngle _scenecapturecomponent2d 9e+01))))

(fn ConstructionScript)