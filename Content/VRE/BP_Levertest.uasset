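; Test actor in the VRE folder that exercises a VR lever component's state-change event.
; Gripping the lever binds a custom handler to the lever's state-changed event, rather than binding at BeginPlay.
; The handler prints a debug "Hello" whenever the reported lever status is true.
; BeginPlay, overlap and Tick are disabled stubs, and the construction script only calls its parent.
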(event OnGripped(Lever)
  (params (GrippingController :type Grip%20Motion%20Controller%20Component%20Object%20Reference) (GripInformation :type BP%20Actor%20Grip%20Information%20Structure%20%28by%20ref%29))
  (EventDispatchers|BindEventtoOnLeverStateChanged (Variables|Default|GetVRLever) (delegate Custom|Lever%20change)))

(event Custom|Lever%20change
  (params (LeverStatus :type Boolean) (LeverStatusType :type EVRInteractibleLeverEventType%20Enum :default "LeverPositive") (LeverAngleAtTime :type Float%20%28single-precision%29) (FullLeverAngleAtTime :type Float%20%28single-precision%29))
  (if LeverStatus
    (Development|PrintString "Hello")))

(event EventBeginPlay
  (|CallParentFunction) ; This node is disabled and will not be called.\nDrag off pins to build functionality.
)

(event Collision|EventActorBeginOverlap
  (params (OtherActor :type Actor%20Object%20Reference))
  (|CallParentFunction OtherActor) ; This node is disabled and will not be called.\nDrag off pins to build functionality.
)

(event EventTick
  (params (DeltaSeconds :type Float%20%28single-precision%29))
  (|CallParentFunction DeltaSeconds) ; This node is disabled and will not be called.\nDrag off pins to build functionality.
)

(fn ConstructionScript
  (|CallParentFunction))